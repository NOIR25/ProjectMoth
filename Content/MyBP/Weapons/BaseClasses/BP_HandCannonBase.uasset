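; Base hand cannon weapon Blueprint that adds a charge-and-release alt fire firing a burst of projectiles.
; Pressing starts a looping timer to build charge toward the weapon data's charge time; releasing picks a burst size from quarter-step charge thresholds.
; A delayed loop spawns each projectile at the active barrel's muzzle, falling back to the weapon's muzzle bone.
; The projectile spread helper's spray-angle calculation is left unconnected.
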(event Custom|AltFire
  (params (isRicochet :type Boolean) (HitActor :type Actor%20Object%20Reference)))

(event Custom|Projectiles
  (params (First%20Index :type Integer) (SecondIndex :type Integer))
  (Utilities|ForLoopwithDelay First%20Index SecondIndex 0.08
    (:Loop%20Body
      (CallFunction|SpawnProjectile))
    (:Completed
      (Utilities|Time|ClearandInvalidateTimerbyHandle (Variables|Default|GetAltFireChargeTimer))
      (Variables|Default|SetChargeSeconds 0.0)
      (Variables|Default|SetChargePercent 0.0))))

(event EventReleaseAltFire
  (Utilities|Time|ClearandInvalidateTimerbyHandle (Variables|Default|GetAltFireChargeTimer))
  (Variables|Default|SetChargeSeconds 0.0)
  (CallFunction|AltFireShoot))

(event EventPressAltFire
  (params (Player :type BP%20First%20Person%20Character%20Object%20Reference) (ShotFromWeapon :type BP%20Weapon%20Class%20Object%20Reference))
  (bind _returnvalue (Utilities|Time|SetTimerbyEvent (EventDispatchers|CreateEvent :!event CallAltFire) 0.01 true))
  (Variables|Default|SetAltFireChargeTimer _returnvalue))

(fn ConstructionScript
  (|CallParentFunction))

(fn CallAltFire
  (bind _output_get (Variables|Default|SetChargeSeconds (+ (Variables|Default|GetChargeSeconds) 0.01)))
  (bind _output_get_2 (Variables|Default|SetChargePercent (/ _output_get (Variables|/Game/MyBP/Weapons/Data/ProceduralWeaponSystem/PDA_WeaponBase.PDA_WeaponBase_C|GetChargeTime (Variables|Default|GetWeaponData)))))
  (Development|PrintString (Utilities|String|ToString(Float) _output_get_2))
  (if (>= _output_get (Variables|/Game/MyBP/Weapons/Data/ProceduralWeaponSystem/PDA_WeaponBase.PDA_WeaponBase_C|GetChargeTime (Variables|Default|GetWeaponData)))
    (Utilities|Time|ClearandInvalidateTimerbyHandle (Variables|Default|GetAltFireChargeTimer))))

(fn AltFireShoot
  (Math|Float|CompareFloat (Variables|Default|GetChargePercent) 0.75
    (:>
      (Development|PrintString "Shoot 4" :!label _label)
      (CallFunction|Projectiles 0 5))
    (:==
      (goto _label))
    (:<
      (Math|Float|CompareFloat (Variables|Default|GetChargePercent) 0.5
        (:>
          (Development|PrintString "Shoot 3" :!label _label_2)
          (CallFunction|Projectiles 0 3))
        (:==
          (goto _label_2))
        (:<
          (Math|Float|CompareFloat (Variables|Default|GetChargePercent) 0.25
            (:>
              (Development|PrintString "Shoot 2" :!label _label_3)
              (CallFunction|Projectiles 0 1))
            (:==
              (goto _label_3))
            (:<
              (Math|Float|CompareFloat (Variables|Default|GetChargePercent) 0.0
                (:==
                  _)
                (:<
                  _))
              (Development|PrintString "Dont Shoot")
              (Utilities|Time|ClearandInvalidateTimerbyHandle (Variables|Default|GetAltFireChargeTimer))
              (Variables|Default|SetChargeSeconds 0.0)
              (Variables|Default|SetChargePercent 0.0))))))))

(fn SpawnProjectile
  (Variables|Default|GetActiveBarrel
    (:then
      (Game|SpawnActorfromClass "/Game/MyBP/Actor/Projectile/BP_Projectile.BP_Projectile_C" (Math|Transform|MakeTransform (+ (.location (Transformation|GetWorldTransform (Variables|/Game/MyBP/Weapons/AttachmentClasses/BP_AttachmentClass.BP_AttachmentClass_C|GetMuzzleFlashPoint (Variables|Default|GetActiveBarrel)))) "20.000000,0.000000,0.000000") (Utilities|ProjectileSpread 5.0) "1.000000,1.000000,1.000000") "Undefined" "MultiplyWithRoot" 0 self 0))
    (:else
      (Game|SpawnActorfromClass "/Game/MyBP/Actor/Projectile/Throwables/BP_Projectile.BP_Projectile_C" (Math|Transform|MakeTransform (.location (Transformation|GetBoneTransform (Variables|Default|GetMyWeapon) "MuzzlePoint" "RTS_World")) (Utilities|ProjectileSpread 5.0) "1.000000,1.000000,1.000000") "Undefined" "MultiplyWithRoot" 0 self 0))))