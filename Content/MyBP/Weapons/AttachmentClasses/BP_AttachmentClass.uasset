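; Base class for weapon attachments, providing an alt-fire interface and a randomly assigned elemental type.
; Press, hold and release events forward to empty AltFire functions that serve as override hooks, with press also storing the Player.
; BeginPlay picks one of four power-of-two elements at random and maps it to ElementalFlagType.
; CooldownAltFire clears the OnCooldown gameplay tag; nothing here adds it.
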(event Custom|CooldownAltFire
  (GameplayTags|RemoveGameplayTag (Variables|Default|GetGameplayTag) "(TagName=\"Attachments.AltFire.OnCooldown\")" :!class /Script/GameplayTags.BlueprintGameplayTagLibrary))

(event EventBeginPlay
  (CallFunction|AssignElementalFlags))

(event EventHoldAltFire
  (CallFunction|AltFireHeld))

(event EventReleaseAltFire
  (CallFunction|AltFireReleased))

(event EventPressAltFire
  (params (Player :type BP%20First%20Person%20Character%20Object%20Reference) (ShotFromWeapon :type BP%20Weapon%20Class%20Object%20Reference))
  (bind _output_get (Variables|Default|SetPlayer Player))
  (CallFunction|AltFirePressed _output_get ShotFromWeapon))

(fn ConstructionScript)

(fn AltFirePressed
  (params (Player :type BP%20First%20Person%20Character%20Object%20Reference) (ShotFromWeapon :type BP%20Weapon%20Class%20Object%20Reference)))

(fn AltFireReleased)

(fn AltFireHeld)

(fn RandomiseElement
  (switch int (Math|Random|RandomIntegerinRange 0 3)
    (:0
      (Variables|Default|SetElementalType "NewEnumerator0"))
    (:1
      (Variables|Default|SetElementalType "NewEnumerator1"))
    (:2
      (Variables|Default|SetElementalType "NewEnumerator2"))
    (:3
      (Variables|Default|SetElementalType "NewEnumerator3")))
  (return))

(fn AssignElementalFlags
  (CallFunction|RandomiseElement)
  (Variables|Default|SetElementalFlagType (Utilities|Select :Index (Variables|Default|GetElementalType) :NewEnumerator0 1 :NewEnumerator1 2 :NewEnumerator2 4 :NewEnumerator3 8)))