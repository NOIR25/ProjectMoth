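; BP_WaveSpawner is a spawn point that releases queued wave enemies at its own transform.
; Once handed a wave manager, it starts a looping timer on the manager's SpawnDelay to drive spawning.
; Each spawn takes the front class from the manager's EnemyQueue and binds its death event, with defeats relayed to the manager.
; Newly queued enemies spawn immediately unless an AI overlaps its sphere, though the queue's front goes first.
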(event Custom|TryToSpawn
  (CallFunction|SpawnEnemy))

(event Custom|StartProcesses
  (bind _returnvalue (Utilities|Time|SetTimerbyEvent (EventDispatchers|CreateEvent :!event Custom|TryToSpawn) (Variables|/Game/MyBP/WaveData/WaveSystem/BP_WaveMaster.BP_WaveMaster_C|GetSpawnDelay (Variables|Default|GetWave%20Manager%20Class)) true))
  (Variables|Default|SetSpawnLoopTimer _returnvalue))

(event Custom|OnEnemyDefeated
  (Default|OnEnemyDefeated (Variables|Default|GetWave%20Manager%20Class)))

(event EventFetchWaveManager
  (params (WaveManagerClass :type BP%20Wave%20Master%20Object%20Reference))
  (Variables|Default|SetWave%20Manager%20Class WaveManagerClass)
  (CallFunction|StartProcesses))

(fn ConstructionScript)

(fn SpawnEnemy
  (if (Utilities|Array|IsValidIndex (Variables|/Game/MyBP/WaveData/WaveSystem/BP_WaveMaster.BP_WaveMaster_C|GetEnemyQueue (Variables|Default|GetWave%20Manager%20Class)))
    (bind _returnvalue (Game|SpawnActorfromClass (Utilities|Array|Get(acopy) (Variables|/Game/MyBP/WaveData/WaveSystem/BP_WaveMaster.BP_WaveMaster_C|GetEnemyQueue (Variables|Default|GetWave%20Manager%20Class))) (Transformation|GetActorTransform) "AdjustIfPossibleButAlwaysSpawn" "MultiplyWithRoot" 0 0))
    (EventDispatchers|BindEventtoOnDeath _returnvalue (EventDispatchers|CreateEvent :!event Custom|OnEnemyDefeated))
    (Utilities|Array|RemoveIndex (Variables|/Game/MyBP/WaveData/WaveSystem/BP_WaveMaster.BP_WaveMaster_C|GetEnemyQueue (Variables|Default|GetWave%20Manager%20Class)))
    (return true)
    (else
      (return false))))

(fn AddEnemytoQueue
  (params (EnemyClass :type BP%20AI%20Master%20Class%20Reference%20%28by%20ref%29))
  (Utilities|Array|Add (Variables|/Game/MyBP/WaveData/WaveSystem/BP_WaveMaster.BP_WaveMaster_C|GetEnemyQueue (Variables|Default|GetWave%20Manager%20Class)) EnemyClass)
  (if (Utilities|Array|IsValidIndex (Collision|GetOverlappingActors (Variables|Default|GetSphere) "/Game/MyBP/Actor/Enemies/BP_AIMaster.BP_AIMaster_C" :!class /Script/Engine.PrimitiveComponent))
    (return)
    (else
      (CallFunction|SpawnEnemy)
      (return))))

(fn GetInventoryStats
  (return))

(fn IsPlayerInputEnabled?
  (return false))