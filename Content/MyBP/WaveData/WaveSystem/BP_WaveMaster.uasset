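; Wave manager that runs escalating enemy rounds with timed intermissions, game mode notifications and on-screen debug stats.
; A curve table scales spawn budget and concurrent enemy cap by wave.
; Mutually recursive functions spend the budget on random data-asset enemies under a cost cap, or one mini boss every fifth wave.
; Random spawners queue random pool picks, topped up upon kills until the round ends.
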(event EventBeginPlay
  (Classes|ClassFetcher)
  (CallFunction|AssignWaveManagertoSpawners)
  (EventCalls|CallRoundStart)
  (Input|EnableInput (Game|GetPlayerController 0)))

(event EventTick
  (params (DeltaSeconds :type Float%20%28single-precision%29))
  (Development|PrintText (Utilities|Text|FormatText "Wave - {Wave} 
Enemies Remaining - {ER} 
Max Enemy at once - {MEAO}" (Variables|WaveTracking|GetCurrentWave) (Variables|Default|GetEnemyRemaining) (Variables|Default|GetEnemyMaxCount)) true true "(R=0.134277,G=1.000000,B=0.000000,A=1.000000)" 0.0)
  (Development|PrintText (Utilities|Text|FormatText "Enemy Pool Size : {EQ}" (Utilities|Array|Length (Variables|Default|GetWavePool))) true true "(R=0.896378,G=0.201102,B=1.000000,A=1.000000)" 0.0)
  (Development|PrintString (Utilities|String|ToString(Float) (Variables|Default|GetDifficultyMultiplier)) true true "(R=1.000000,G=0.102237,B=0.072390,A=1.000000)" 0.0))

(event Input|KeyboardEvents|3
  (params (Key :type Key%20Structure))
  (:Pressed
    (EventCalls|CallRoundStart)))

(fn ConstructionScript)

(fn CallRoundEnd
  (params (IntermissionTime :type Float%20%28double-precision%29))
  (bind _returnvalue (Utilities|Time|SetTimerbyFunctionName 0 "CallRoundStart" IntermissionTime))
  (Variables|Default|SetIntermissionTimer _returnvalue)
  (Class|BPIGlobalEvents|EndRound(Message) (Variables|FetchedClasses|GetMy%20Gamemode)))

(fn CallIntermissionStart
  (Default|CallOnIntermissionStart (Variables|FetchedClasses|GetMy%20Gamemode)))

(fn CallIntermissionEnd
  (Default|CallOnIntermissionEnd (Variables|FetchedClasses|GetMy%20Gamemode)))

(fn CallRoundStart
  (bind _currentwave (Variables|WaveTracking|GetCurrentWave))
  (CallFunction|ScaleDifficulty)
  (CallFunction|ClearWaveQueue)
  ;[1 1 1] Is the next wave a boss wave
  (Math|Integer|IncrementInt _currentwave
    (:%20%20
      (if (== (Math|Integer|%(Integer) _currentwave 5) 0)
        (Variables|Default|SetBossWave true)
        (else
          (Variables|Default|SetBossWave false)))
      (CallFunction|SetEnemyData)
      (CallFunction|CheckSpawnBudget)
      (for _index (range 0 (- (Math|Integer|Min(Integer) (CallFunction|GetPoolSize) (Variables|Default|GetEnemyMaxCount)) 1))
        (bind _enemy_class (CallFunction|GetEnemyfromPool))
        (Default|AddEnemytoQueue (.OutItem (Utilities|Array|Random (Variables|WaveData|GetSpawners))) _enemy_class))
      (Class|BPIGlobalEvents|NewRound(Message) (Variables|FetchedClasses|GetMy%20Gamemode) (Variables|Default|GetEnemyRemaining) (Variables|WaveTracking|GetCurrentWave)))))

(fn ClassFetcher
  (bind _mygamemode (CallFunction|GetGM))
  (Variables|FetchedClasses|SetMy%20Gamemode _mygamemode))

(fn AssignWaveManagertoSpawners
  (bind _outactors (Actor|GetAllActorsOfClass "/Game/MyBP/WaveData/WaveSystem/BP_WaveSpawner.BP_WaveSpawner_C"))
  (bind _output_get (Variables|WaveData|SetSpawners _outactors))
  (for _array_element _output_get
    (Class|BPIGlobalEvents|FetchWaveManager(Message) _array_element self))
  (return))

(fn OnEnemyDefeated
  (bind _result (Math|Integer|DecrementInt (Variables|Default|GetEnemyRemaining))
    (:%20%20
      (Class|BPIGlobalEvents|WaveEnemyKilled(Message) (Variables|FetchedClasses|GetMy%20Gamemode) _result)
      (if (< (Variables|Default|GetEnemyRemaining) (Variables|Default|GetEnemyMaxCount))
        (if (<= (Variables|Default|GetEnemyRemaining) 0)
          (EventCalls|CallRoundEnd 5.0))
        (else
          (bind _enemy_class (CallFunction|GetEnemyfromPool))
          (Default|AddEnemytoQueue (.OutItem (Utilities|Array|Random (Variables|WaveData|GetSpawners))) _enemy_class))))))

(fn IncrementWave
  (return (+ (Variables|WaveTracking|GetCurrentWave) 1)))

(fn GenerateSpawnPool
  (bind (_enemytypes _class _cost) (Utilities|GetEnemyStruct))
  (bind (_enemytypes_2 _class_2) (Utilities|GetEnemyStruct))
  (if (not (Variables|Default|GetBossWave))
    (Utilities|Array|Shuffle (.EnemyTypes (Utilities|GetEnemyStruct)))
    (if (> (Math|Float|Clamp(Float) (* (Variables|Default|GetSpawnBudget) 0.5) 2.0 9999.0) (.Cost (Utilities|GetEnemyStruct)))
      (Variables|Default|SetSpawnBudget (- (Variables|Default|GetSpawnBudget) _cost))
      (Utilities|Array|Add (Variables|Default|GetWavePool) _class)
      (CallFunction|CheckSpawnBudget)
      (else
        (CallFunction|CheckSpawnBudget)))
    (else
      ;[1 1 1] Select Mini Boss
      (Utilities|Array|Shuffle _enemytypes_2)
      (Utilities|Array|Add (Variables|Default|GetWavePool) _class_2)
      (Variables|Default|SetSpawnBudget 0)
      (return))))

(fn CheckSpawnBudget
  (if (> (Variables|Default|GetSpawnBudget) 0)
    (CallFunction|GenerateSpawnPool)
    (else
      (Variables|Default|SetEnemyRemaining (CallFunction|GetPoolSize))
      (return))))

(fn GetPoolSize
  (return (Utilities|Array|Length (Variables|Default|GetWavePool))))

(fn GetEnemyfromPool
  (bind _wavepool (Variables|Default|GetWavePool))
  (Utilities|Array|Shuffle _wavepool)
  (bind _output_get (LocalVariables|SetL_EnemyToPick (Utilities|Array|Get(acopy) _wavepool)))
  (return _output_get))

(fn ClearWaveQueue
  (Utilities|Array|Clear (Variables|Default|GetWavePool)))

(fn ScaleDifficulty
  (bind _wavecurvetable (Variables|Default|GetWaveCurveTable))
  (bind _outxy (DataTable|EvaluateCurveTableRow (.curvetable _wavecurvetable) (.rowname _wavecurvetable) (Math|Conversions|ToFloat(Integer) (Variables|WaveTracking|GetCurrentWave)))
    (:RowFound
      (Variables|Default|SetDifficultyMultiplier _outxy)
      (Variables|Default|SetSpawnBudget (Math|Float|Truncate (* (Variables|Default|GetSpawnBudgetBase) (Variables|Default|GetDifficultyMultiplier))))
      (Variables|Default|SetEnemyMaxCount (Math|Float|Truncate (* (Variables|Default|GetEnemyMaxCountBase) (Variables|Default|GetDifficultyMultiplier)))))
    (:RowNotFound
      _))
  (return))

(fn SetEnemyData
  (if (Variables|Default|GetBossWave)
    (Variables|Default|SetEnemyData "/Game/MyBP/WaveData/WaveSystem/DA_MiniBossTypes.DA_MiniBossTypes")
    (else
      (Math|Integer|CompareInt (Variables|WaveTracking|GetCurrentWave)
        (:>
          (Variables|Default|SetEnemyData "/Game/MyBP/WaveData/WaveSystem/DA_EnemyTypes.DA_EnemyTypes"))))))