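; BP_Capture is a painting actor that renders brush hits on BP_AIMaster characters through a scene capture.
; On BeginPlay it creates an M_Unwrap material instance, writes capture size and unwrap location to MPC_Global, then clears RT_Capture after a short delay.
; PaintActor swaps the mesh's first material to the unwrap instance, sets hit location and brush radius, then captures.
; The original material is saved, but its restore step is unconnected.
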(event EventBeginPlay
  (Utilities|InitialiseParameters)
  (bind _returnvalue (Rendering|Material|CreateDynamicMaterialInstance "/Game/M_/Testing/M_Unwrap.M_Unwrap" "None" "None" :!class /Script/Engine.KismetMaterialLibrary))
  (Variables|Default|SetUnwrapMaterial _returnvalue))

(fn ConstructionScript)

(fn PaintActor
  (params (ActorToPaint :type Actor%20Object%20Reference) (HitLocation :type Vector) (Brush%20Radius :type Float%20%28double-precision%29))
  (bind _asbp_aimaster (Utilities|Casting|CastToBP_AIMaster ActorToPaint))
  (Variables|Default|SetMesh%20Component (Variables|/Script/Engine.Character|GetMesh _asbp_aimaster))
  (Utilities|FlowControl|Sequence
    (:then_0
      (Variables|Default|SetOriginalMaterial (Rendering|Material|GetMaterial (Variables|Default|GetMesh%20Component) 0))
      (Rendering|Material|SetMaterial (Variables|Default|GetMesh%20Component) 0 (Variables|Default|GetUnwrapMaterial)))
    (:then_1
      (Rendering|Material|SetVectorParameterValue (Variables|Default|GetUnwrapMaterial) "HitLocation" (Math|Conversions|ToLinearColor(Vector) HitLocation) :!class /Script/Engine.MaterialInstanceDynamic)
      (Rendering|Material|SetScalarParameterValue (Variables|Default|GetUnwrapMaterial) "BrushRadius" Brush%20Radius :!class /Script/Engine.MaterialInstanceDynamic))
    (:then_2
      (Rendering|SceneCapture|CaptureScene (Variables|Default|GetScene%20Capture) :!class /Script/Engine.SceneCaptureComponent2D))))