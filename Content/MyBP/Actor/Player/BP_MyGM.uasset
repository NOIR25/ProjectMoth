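; Game mode that runs combat combo scoring, relays wave round events and hooks into game-instance saving, though its save-data functions are stubs.
; Kills raise a multiplier by amounts set from player and enemy movement tags, scaling score and setting a rank from Basic to God.
; A looping timer decays the combo, faster when the player stands still, and pauses briefly after kills.
; WaveEnd converts combat score into gold stars and resets it.
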(event Custom|On%20First%20Login
  (CallFunction|SaveGMData true))

(event Custom|OnGameLoad
  (SaveGame|InitialiseSaveData)
  (CallFunction|SaveGMData true))

(event Custom|SaveGMData
  (params (Async :type Boolean))
  (bind _gmsave (SaveGame|GetGMSave))
  (Class|BPISaveGame|SaveGamemode(Message) (Game|GetGameInstance) _gmsave Async))

(event Custom|SaveLastData
  (CallFunction|SaveGMData true))

(event Custom|DecayCombo
  ;[1 1 1] Decay Combo Score
  (|DecayComboSystem))

(event Custom|ResumeComboDecay
  ;[1 1 1] Try to resume combo decay
  (bind _result (Math|Float|IncrementFloat (Variables|ComboSystem|GetComboTimerPosition))
    (:%20%20
      (if (>= _result 3.0)
        (Utilities|Time|UnpauseTimerbyHandle (Variables|ComboSystem|GetComboTimer))))))

(event EventTick
  (params (DeltaSeconds :type Float%20%28single-precision%29)))

(event EventEnemyFelled
  (params (Class :type E_EnemyType%20Enum :default "NewEnumerator0") (Enemy :type BP%20AI%20Master%20Object%20Reference) (EnemiesRemaining :type Integer))
  (|ComboSystem Enemy))

(event EventBeginPlay
  (Initialisation|FetchClasses)
  (Initialisation|BindtoDispatchers)
  (SaveGame|InitialiseSaveData)
  (bind _returnvalue (Utilities|Time|SetTimerbyEvent (EventDispatchers|CreateEvent :!event Custom|DecayCombo) (Variables|ComboSystem|GetComboDecaySpeed) true))
  (Variables|ComboSystem|SetComboTimer _returnvalue))

(event EventEndRound
  ;[1 1 1] Wave System
  (Default|CallOnRoundEnd)
  (Default|CallOnIntermissionStart))

(event EventNewRound
  (params (EnemiesRemaining :type Integer) (Wave :type Integer))
  ;[1 1 1] Wave System
  (Variables|Default|SetEnemies%20Remaining EnemiesRemaining)
  (Variables|Default|SetWave Wave)
  (Default|CallOnRoundStart)
  (Default|CallOnIntermissionEnd))

(event EventWaveEnemyKilled
  (params (EnemiesRemaining :type Integer))
  ;[1 1 1] Wave System
  (Variables|Default|SetEnemies%20Remaining EnemiesRemaining)
  (Default|CallOnEnemyFelled))

(fn ConstructionScript)

(fn BindtoDispatchers
  (bind _mygi (Variables|FetchedClasses|GetMyGI)
    (:then
      (EventDispatchers|BindEventtoOnGameLoaded _mygi (EventDispatchers|CreateEvent :!event Custom|OnGameLoad))
      (EventDispatchers|BindEventtoOnRoundEnd (EventDispatchers|CreateEvent :!event WaveEnd)))
    (:else)))

(fn FetchClasses
  (bind _mycontroller (CallFunction|GetPC))
  (Variables|FetchedClasses|SetMy%20Controller _mycontroller)
  (bind _mygameinstance (CallFunction|GetGI))
  (Variables|FetchedClasses|SetMyGI _mygameinstance)
  (bind _myplayer (CallFunction|GetPlayer))
  (Variables|Default|SetMy%20Player _myplayer))

(fn UseGMSave
  (params (GMSave :type S%20Primary%20Save%20Data%20Structure)))

(fn InitialiseSaveData
  ;[0.4583 0.3333 0.1789] Fetches saved data if valid and sets this classes variables to our saved data
  (bind _savegamedata (Class|BPISaveGame|GetGameData(Message) (Game|GetGameInstance)))
  (Utilities|IsValid _savegamedata
    (:Is%20Valid
      (SaveGame|UseGMSave (Variables|/Game/MyBP/SaveGame/BP_SaveGame.BP_SaveGame_C|GetPrimary%20Save%20Data _savegamedata)))))

(fn GetGMSave
  (return ""))

(fn SetComboState
  (CallFunction|SetComboMultiplier)
  (Math|Float|CompareFloat (Variables|ComboSystem|GetComboMultiplier) 2.0
    (:>
      (Variables|ComboSystem|SetComboState "NewEnumerator1" :!label _label)
      (Math|Float|CompareFloat (Variables|ComboSystem|GetComboMultiplier) 3.0
        (:>
          (Variables|ComboSystem|SetComboState "NewEnumerator2" :!label _label_2)
          (Math|Float|CompareFloat (Variables|ComboSystem|GetComboMultiplier) 4.0
            (:>
              (Variables|ComboSystem|SetComboState "NewEnumerator3" :!label _label_3)
              (Math|Float|CompareFloat (Variables|ComboSystem|GetComboMultiplier) 6.0
                (:>
                  (Variables|ComboSystem|SetComboState "NewEnumerator4" :!label _label_4)
                  (Math|Float|CompareFloat (Variables|ComboSystem|GetComboMultiplier) 8.0
                    (:>
                      (Variables|ComboSystem|SetComboState "NewEnumerator5" :!label _label_5)
                      (Math|Float|CompareFloat (Variables|ComboSystem|GetComboMultiplier) 1e+01
                        (:>
                          (Variables|ComboSystem|SetComboState "NewEnumerator6" :!label _label_6))
                        (:==
                          (goto _label_6))
                        (:<
                          _)))
                    (:==
                      (goto _label_5))
                    (:<
                      _)))
                (:==
                  (goto _label_4))
                (:<
                  _)))
            (:==
              (goto _label_3))
            (:<
              _)))
        (:==
          (goto _label_2))
        (:<
          _)))
    (:==
      (goto _label))
    (:<
      (Variables|ComboSystem|SetComboState "NewEnumerator0")))
  (return))

(fn SetComboMultiplier)

(fn CheckPlayerComboTags
  (Utilities|FlowControl|Sequence
    (:then_0
      (Utilities|FlowControl|DoOnce false
        (:Completed
          (LocalVariables|SetL-DefaultAddToCM (Variables|ComboSystem|GetAddToCM)))))
    (:then_1
      (bind _my_player (Variables|Default|GetMy%20Player)
        (:then
          (if (GameplayTags|HasTag (Variables|/Game/FirstPerson/Blueprints/BP_FirstPersonCharacter.BP_FirstPersonCharacter_C|GetGameplayTags _my_player) "(TagName=\"ComboBuffs.Movement\")")
            (|SwitchGameplayTagContainer (Variables|/Game/FirstPerson/Blueprints/BP_FirstPersonCharacter.BP_FirstPersonCharacter_C|GetGameplayTags (Variables|Default|GetMy%20Player))
              (:%28GameplayTags=%28%28TagName="ComboBuffs.Movement.Sliding"%29%29%29
                (Development|PrintString "Sliding")
                (Variables|ComboSystem|SetAddToCM 0.3))
              (:%28GameplayTags=%28%28TagName="ComboBuffs.Movement.GroundSlamming"%29%29%29
                (Development|PrintString "GroundSlamming")
                (Variables|ComboSystem|SetAddToCM 0.6))
              (:%28GameplayTags=%28%28TagName="ComboBuffs.Movement.WallSliding"%29%29%29
                (Development|PrintString "WallSliding")
                (Variables|ComboSystem|SetAddToCM 0.75)))
            (else
              (Variables|ComboSystem|SetAddToCM 0.25)))
          (return))
        (:else)))))

(fn CheckEnemyComboTags
  (params (Enemy :type BP%20AI%20Master%20Object%20Reference))
  (Utilities|FlowControl|Sequence
    (:then_1
      (if (GameplayTags|HasTag (Variables|/Game/MyBP/Actor/Enemies/BP_AIMaster.BP_AIMaster_C|GetGameplayTags Enemy) "(TagName=\"ComboBuffs.Movement\")")
        (|SwitchGameplayTagContainer (Variables|/Game/MyBP/Actor/Enemies/BP_AIMaster.BP_AIMaster_C|GetGameplayTags Enemy)
          (:%28GameplayTags=%28%28TagName="ComboBuffs.Movement.EnemyLifted"%29%29%29
            (Development|PrintString "Lifted")
            (Variables|ComboSystem|SetAddToCM 0.8))))
      (return))))

(fn WaveEnd
  (Variables|Currency|SetGoldStars (Math|Float|Truncate (/ (Variables|ComboSystem|GetCombatScore) 1e+02)))
  (Variables|ComboSystem|SetTotalCombatScore (Variables|ComboSystem|GetCombatScore))
  (Variables|ComboSystem|SetCombatScore 0.0)
  (Variables|ComboSystem|SetComboMultiplier 0.0))

(fn CheckNumpadEntry
  (return false 0))

(fn GetMyGI
  (return 0))

(fn GetMyGM
  (return self))

(fn GetMyHUD
  (return 0))

(fn GetMyPC
  (return 0))

(fn GetMyPlayer
  (return 0))

(fn GetPlayerComponents
  (return 0))

(fn IsPlayerInputEnabled?
  (return false))