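; Wave manager actor that runs the game's cycle of timed intermissions and enemy rounds through GameMode event dispatchers.
; During rounds, a self-rearming timer picks a random spawn point and enemy type (Hider, Runner or Tank), spawning only under that type's cap.
; Round setup scales caps by round number, fixed after round 10, and sums them into the kill goal.
; Tick publishes the current wave and ends the round when kills match that goal.
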(event Custom|CallEnemySpawn
  ;[1 1 1] Enemy Spawn
  (if (Variables|Default|GetroundEnabled)
    (Utilities|Time|SetTimerbyEvent (delegate Custom|CallEnemySpawn) (Variables|Default|GetspawnerTimer) false true)
    (CallFunction|SpawnEnemy (Transformation|GetActorTransform (.OutItem (Utilities|Array|Random (Variables|Default|GetEnemySpawns)))))))

(event Custom|IntermissionStart
  ;[1 1 1] Intermission
  (Development|PrintString "Intermission Start")
  (Utilities|Time|SetTimerbyEvent (delegate Custom|IntermissionEnd) (Variables|Default|GetintermissionTimer)))

(event Custom|IntermissionEnd
  ;[1 1 1] Intermission
  (Development|PrintString "Intermission End" true true "(R=0.847223,G=1.000000,B=0.000000,A=1.000000)")
  (Math|Integer|IncrementInt (Variables|Default|GetcurrentRound)
    (:%20%20
      (CallFunction|SetRoundStart)
      (Default|CallOnRoundStart (Variables|Default|GetMy%20Gamemode)))))

(event Custom|RoundStart
  ;[0.4375 0.4375 0.4375] Round
  (Development|PrintString "Round Start" true true "(R=1.000000,G=0.000000,B=0.053326,A=1.000000)")
  (Development|PrintString (Utilities|String|ToString(Integer) (Variables|Default|GetcurrentRound)) true true "(R=1.000000,G=0.000000,B=0.023145,A=1.000000)")
  (Utilities|Time|SetTimerbyEvent (EventDispatchers|CreateEvent :!event Custom|CallEnemySpawn) (Variables|Default|GetspawnerTimer) false true 3.0)
  (Variables|Default|SetroundEnabled true))

(event Custom|RoundEnd
  ;[0.4375 0.4375 0.4375] Round
  (Development|PrintString "Round End" true true "(R=0.000000,G=1.000000,B=0.008406,A=1.000000)")
  (Variables|Default|SetroundEnabled false)
  (Default|CallOnIntermissionStart (Variables|Default|GetMy%20Gamemode)))

(event Custom|GameOver
  (Development|PrintString "Game Over")
  (Variables|Default|SetroundEnabled false))

(event EventBeginPlay
  (bind _outactors (Actor|GetAllActorsOfClass "/Game/MyBP/Actor/Enemies/BP_EnemySpawn.BP_EnemySpawn_C"))
  (Variables|Default|SetEnemySpawns _outactors)
  (bind _mygamemode (CallFunction|GetGM))
  (bind _output_get (Variables|Default|SetMy%20Gamemode _mygamemode))
  (EventDispatchers|BindEventtoOnIntermissionStart _output_get (EventDispatchers|CreateEvent :!event Custom|IntermissionStart))
  (EventDispatchers|AssignOnIntermissionEnd _output_get (EventDispatchers|CreateEvent :!event Custom|IntermissionEnd))
  (EventDispatchers|BindEventtoOnRoundStart _output_get (EventDispatchers|CreateEvent :!event Custom|RoundStart))
  (EventDispatchers|BindEventtoOnRoundEnd _output_get (EventDispatchers|CreateEvent :!event Custom|RoundEnd))
  (EventDispatchers|BindEventtoOnGameOver _output_get (EventDispatchers|CreateEvent :!event Custom|GameOver))
  (Utilities|FlowControl|Delay 0.2)
  (Default|CallOnIntermissionStart _mygamemode))

(event EventTick
  (params (DeltaSeconds :type Float%20%28single-precision%29))
  (bind _my_gamemode (Variables|Default|GetMy%20Gamemode))
  (Variables|/Game/MyBP/Actor/Player/BP_MyGM.BP_MyGM_C|SetCurrentWAVE (Variables|Default|GetMy%20Gamemode) (Variables|Default|GetcurrentRound))
  (Development|PrintString (Utilities|String|ToString(Boolean) (Variables|Default|GetroundEnabled)) true true "(R=0.000000,G=0.660000,B=1.000000,A=1.000000)" 0.0)
  (if (Variables|Default|GetroundEnabled)
    (if (== (Variables|/Game/MyBP/Actor/Player/BP_MyGM.BP_MyGM_C|GetKillsThisRound _my_gamemode) (Variables|/Game/MyBP/Actor/Player/BP_MyGM.BP_MyGM_C|GetKillGoalThisRound _my_gamemode))
      (Default|CallOnRoundEnd (Variables|Default|GetMy%20Gamemode)))))

(fn ConstructionScript)

(fn SpawnEnemy
  (params (SpawnLocation :type Transform))
  (switch int (Math|Random|RandomInteger 3)
    (:Default
      (Development|PrintString "SPAWN FAILED!" true true "(R=1.000000,G=0.000000,B=0.005162,A=1.000000)"))
    (:0
      (if (< (Variables|Default|GethidersSpawned) (Variables|Default|GetmaxHidersRound))
        (Variables|Default|SetSelectedEnemy 0)
        (Math|Integer|IncrementInt (Variables|Default|GethidersSpawned)
          (:%20%20
            (Game|SpawnActorfromClass (Utilities|Array|Get(acopy) (Variables|Default|GetEnemies) (Variables|Default|GetSelectedEnemy)) SpawnLocation "Undefined" "MultiplyWithRoot" 0 0 :!label _label)))))
    (:1
      (if (< (Variables|Default|GetrunnersSpawned) (Variables|Default|GetmaxRunnersRound))
        (Variables|Default|SetSelectedEnemy 1)
        (Math|Integer|IncrementInt (Variables|Default|GetrunnersSpawned)
          (:%20%20
            (goto _label)))))
    (:2
      (if (< (Variables|Default|GettanksSpawned) (Variables|Default|GetmaxTanksRound))
        (Variables|Default|SetSelectedEnemy 2)
        (Math|Integer|IncrementInt (Variables|Default|GettanksSpawned)
          (:%20%20
            (goto _label)))))))

(fn SetRoundStart
  (Variables|/Game/MyBP/Actor/Player/BP_MyGM.BP_MyGM_C|SetKillsThisRound (Variables|Default|GetMy%20Gamemode) 0)
  (Variables|Default|SethidersSpawned 0)
  (Variables|Default|SetrunnersSpawned 0)
  (Variables|Default|SettanksSpawned 0)
  (if (<= (Variables|Default|GetcurrentRound) 10)
    (Variables|Default|SetmaxHidersRound 5)
    (if (> (Variables|Default|GetcurrentRound) 1)
      (Variables|Default|SetmaxRunnersRound (* 2 (Variables|Default|GetcurrentRound)))
      (if (> (Variables|Default|GetcurrentRound) 3)
        (Variables|Default|SetmaxTanksRound 1)))
    (else
      (Variables|Default|SetmaxHidersRound 5)
      (Variables|Default|SetmaxRunnersRound 20)
      (Variables|Default|SetmaxTanksRound 2)))
  (Variables|/Game/MyBP/Actor/Player/BP_MyGM.BP_MyGM_C|SetKillGoalThisRound (Variables|Default|GetMy%20Gamemode) (+ (Variables|Default|GetmaxHidersRound) (Variables|Default|GetmaxRunnersRound) (Variables|Default|GetmaxTanksRound))))

(fn SetRoundEnd)