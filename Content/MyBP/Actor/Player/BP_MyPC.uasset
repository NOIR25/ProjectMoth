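; BP_MyPC is a player controller that registers the default input controls at game start.
; On BeginPlay it adds IMC_Default to the Enhanced Input local player subsystem after a validity check.
; Its getters for game instance, game mode, HUD, controller, player and components are empty stubs.
; GetMyPC holds a return of self, but that node is unconnected and never runs.
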(event EventBeginPlay
  (bind _returnvalue (PlayerController|LocalPlayerSubsystems|GetEnhancedInputLocalPlayerSubsystem))
  ;[0 0 0] Create / Add Input Controls
  (Utilities|IsValid _returnvalue
    (:Is%20Valid
      (Input|AddMappingContext _returnvalue "/Game/MyBP/Input/IMC_Default.IMC_Default" 0 "(bIgnoreAllPressedKeysUntilRelease=True,bForceImmediately=False,bNotifyUserSettings=False)"))))

(fn ConstructionScript)

(fn GetMyGI
  (return 0))

(fn GetMyGM
  (return 0))

(fn GetMyHUD
  (return 0))

(fn GetMyPC)

(fn GetMyPlayer
  (return 0))

(fn GetPlayerComponents
  (return 0))