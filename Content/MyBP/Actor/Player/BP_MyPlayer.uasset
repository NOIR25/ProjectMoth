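; Player Blueprint that caches game references, tracks a holding state and provides hooks for save data.
; BeginPlay runs ClassFetcher to store the game instance and HUD, and the F key deletes save data through the game instance.
; InitialiseSaveData passes valid primary save data to an empty UsePlayerSave event, but nothing here calls it.
; The numpad check and remaining getters are stubs returning defaults or nothing.
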(event Custom|UsePlayerSave
  (params (PrimarySaveData :type S%20Primary%20Save%20Data%20Structure)))

(event EventBeginPlay
  (CallFunction|ClassFetcher))

(event EventSetPlayerHolding
  (params (Holding :type Boolean))
  (Variables|Default|SetIsHolding Holding))

(event Input|KeyboardEvents|F
  (params (Key :type Key%20Structure :default "None"))
  (:Pressed
    (Class|BPISaveGame|DeleteSaveData(Message) (Variables|Default|GetMy%20Game%20Instance))))

(fn ConstructionScript)

(fn ClassFetcher
  (bind _mygameinstance (CallFunction|GetGI))
  (Variables|Default|SetMy%20Game%20Instance _mygameinstance)
  (bind _hud (CallFunction|GetHUD))
  (Variables|Default|SetHUD _hud))

(fn InitialiseSaveData
  ;[0.4688 0.3558 0.1758] Fetches saved data if valid and sets this classes variables to our saved data
  (bind _savegamedata (Class|BPISaveGame|GetGameData(Message) (Variables|Default|GetMy%20Game%20Instance)))
  (Utilities|IsValid _savegamedata
    (:Is%20Valid
      (CallFunction|UsePlayerSave (Variables|/Game/MyBP/SaveGame/BP_SaveGame.BP_SaveGame_C|GetPrimary%20Save%20Data _savegamedata)))))

(fn CheckNumpadEntry
  (return false 0))

(fn GetMyGI
  (return 0))

(fn GetMyGM
  (return 0))

(fn GetMyHUD
  (return 0))

(fn GetMyPC
  (return 0))

(fn GetMyPlayer
  (return 0))

(fn GetPlayerComponents
  (return 0))