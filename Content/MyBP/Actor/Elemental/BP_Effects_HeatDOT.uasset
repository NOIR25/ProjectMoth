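; Heat damage-over-time effect actor that hurts the actor it is attached to.
; On BeginPlay it applies damage at once, starts a looping timer to repeat ticks every couple of seconds, and calls DestroyCountdown.
; Each DoDOT tick sends a damage info struct to the attach parent through TakeDamageMessage and activates the Niagara effect without resetting it.
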(event Custom|Do%20DOT
  (Class|BPIDamagable|TakeDamage(Message) (Actor|GetAttachParentActor) (Utilities|Struct|MakeS_DamageInfo (Variables|Default|GetDamage) "NewEnumerator4" "NewEnumerator3"))
  (Components|Activation|Activate (Variables|Default|GetNiagara) false))

(event EventBeginPlay
  (CallFunction|DoDOT)
  (Utilities|Time|SetTimerbyEvent (EventDispatchers|CreateEvent :!event Custom|Do%20DOT) 2.0 true)
  (CallFunction|DestroyCountdown))

(fn ConstructionScript
  (|CallParentFunction))