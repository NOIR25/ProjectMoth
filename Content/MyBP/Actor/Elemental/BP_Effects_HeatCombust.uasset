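; Heat combustion effect actor that detonates on BeginPlay and then starts a destroy countdown.
; Combust plays Niagara and sphere-overlaps nearby pawns, excluding itself and the player, sending each a randomized launch, spread damage and a weighted-chance elemental proc.
; The actor it is attached to receives separate AOE damage, with all effects delivered through message calls.
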(event Custom|Combust
  (bind _returnvalue (Math|Random|RandomFloatinRange -5e+02 5e+02))
  (Components|Activation|Activate (Variables|Default|GetNiagara) false)
  (bind _myplayer (CallFunction|GetPlayer))
  (bind _outactors (Collision|SphereOverlapActors (Transformation|GetActorLocation) (Variables|Default|GetAOE%20Radius) (Utilities|Array|MakeArray "ObjectTypeQuery3") 0 (Utilities|Array|MakeArray self _myplayer)))
  (for _array_element _outactors
    (Class|BPIEnemy|LaunchSlam(Message) _array_element (Math|Vector|MakeVector _returnvalue _returnvalue (Math|Random|RandomFloatinRange 2.5e+02 7.5e+02)))
    (Class|BPIEnemy|ProcElementalDamage(Message) _array_element (Math|Random|RandomBoolwithWeight (Variables|Default|GetChanceToSpread)) 1)
    (Class|BPIDamagable|TakeDamage(Message) _array_element (Utilities|Struct|MakeS_DamageInfo (Variables|Default|GetSpreadDamage) "NewEnumerator3" "NewEnumerator4")))
  (Class|BPIDamagable|TakeDamage(Message) (Actor|GetAttachParentActor) (Utilities|Struct|MakeS_DamageInfo (Variables|Default|GetAOEDamage) "NewEnumerator3" "NewEnumerator4")))

(event EventBeginPlay
  (CallFunction|Combust)
  (CallFunction|DestroyCountdown))

(fn ConstructionScript
  (|CallParentFunction))