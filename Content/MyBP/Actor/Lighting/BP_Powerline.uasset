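; Powerline light actor with a configurable spotlight and a tinted billboard bloom sprite that scales with player distance.
; The construction script creates the sprite's dynamic material and applies colour, intensity, cone, shadow and attenuation settings.
; While the player overlaps PlayerDetection, a looping timer enlarges the bloom as distance grows, within a clamped range.
; SetBloomScale rewrites the sprite element and toggles visibility twice to force a runtime refresh.
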(event OnComponentBeginOverlap(PlayerDetection)
  (params (OverlappedComponent :type Primitive%20Component%20Object%20Reference) (OtherActor :type Actor%20Object%20Reference) (OtherComp :type Primitive%20Component%20Object%20Reference) (OtherBodyIndex :type Integer) (bFromSweep :type Boolean) (SweepResult :type Hit%20Result%20Structure%20%28by%20ref%29))
  ;[1 1 1] Overlap and end overlap to trigger distance check timer
  (if (Actor|ActorHasTag OtherActor "Player")
    (bind _returnvalue (Utilities|Time|SetTimerbyEvent (EventDispatchers|CreateEvent :!event CEScaleBLoom) 0.033 true))
    (Variables|Default|SetScaleBloomTimer _returnvalue)))

(event OnComponentEndOverlap(PlayerDetection)
  (params (OverlappedComponent :type Primitive%20Component%20Object%20Reference) (OtherActor :type Actor%20Object%20Reference) (OtherComp :type Primitive%20Component%20Object%20Reference) (OtherBodyIndex :type Integer))
  ;[1 1 1] Overlap and end overlap to trigger distance check timer
  (if (Actor|ActorHasTag OtherActor "Player")
    (Utilities|Time|ClearandInvalidateTimerbyHandle (Variables|Default|GetScaleBloomTimer))))

(event Custom|CE_ScaleBloom
  ;[1 1 1] Timer checks distance to player and scales bloom based on this distance
  (Variables|Default|SetBloomScaleMultiplier (Math|Float|MapRangeClamped (Math|Vector|Distance(Vector) (Transformation|GetActorLocation) (Transformation|GetActorLocation (Variables|Default|GetMy%20Player))) 1.5e+03 5e+02 1.5 1.0))
  (CallFunction|SetBloomScale (* (Variables|Default|GetBloomScale) (Variables|Default|GetBloomScaleMultiplier))))

(event EventBeginPlay
  (bind _myplayer (CallFunction|GetPlayer))
  (Variables|Default|SetMy%20Player _myplayer))

(fn ConstructionScript
  (Variables|Default|GetDynamicMaterial
    (:then
      _)
    (:else
      (CallFunction|CreateMaterialInstance)))
  (CallFunction|SetBloomScale (* (Variables|Default|GetBloomScale) (Variables|Default|GetBloomScaleMultiplier)))
  (Rendering|Components|Light|SetLightColor (Variables|Default|GetSpotLight) (Variables|Default|GetLightColour) true)
  (Rendering|Material|SetVectorParameterValue (Variables|Default|GetDynamicMaterial) "BloomTint" (Variables|Default|GetLightColour) :!class /Script/Engine.MaterialInstanceDynamic)
  (Rendering|Components|Light|SetIntensity (Variables|Default|GetSpotLight) (Variables|Default|GetLightIntensity))
  (Rendering|Lighting|SetOuterConeAngle (Variables|Default|GetSpotLight) (Variables|Default|GetInner%20Cone%20Angle))
  (Rendering|Components|Light|SetCastShadows (Variables|Default|GetSpotLight) (Variables|Default|GetCast%20Shadows))
  (Rendering|Lighting|SetAttenuationRadius (Variables|Default|GetSpotLight) (Variables|Default|GetAttenuation)))

(fn CreateMaterialInstance
  (bind _returnvalue (Rendering|Material|CreateDynamicMaterialInstance (Variables|Default|GetLightFX) 0 0 "None" :!class /Script/Engine.PrimitiveComponent))
  (Variables|Default|SetDynamicMaterial _returnvalue))

(fn SetBloomScale
  (params (NewScale :type Float%20%28double-precision%29))
  (bind _lightfx (Variables|Default|GetLightFX))
  (Utilities|Array|SetArrayElem (Variables|/Script/Engine.MaterialBillboardComponent|GetElements (Variables|Default|GetLightFX)) 0 (Utilities|Struct|MakeMaterialSpriteElement (Variables|Default|GetDynamicMaterial) 0 false NewScale NewScale))
  ;[1 1 1] Refreshes Billboard - otherwise nothing changes at runtime
  (Rendering|ToggleVisibility _lightfx false)
  (Rendering|ToggleVisibility _lightfx false))