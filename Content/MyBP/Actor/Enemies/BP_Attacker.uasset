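; BP_Attacker is an enemy that fires BP_SkipShot projectiles at the player's LookAT point.
; Its movement function faces the player, approaches, backs away or strafes by AttackDistance, and updates IsAttacking.
; Tick uses that flag to start, once, a looping shot timer with a randomized interval, or clear it.
; A self-repeating Strafe event flips direction; neither it nor the movement function is called within this Blueprint.
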(event Custom|Strafe
  ;[1 1 1] Strafe
  (bind _isa (Utilities|FlowControl|FlipFlop)
    (:A
      _)
    (:B
      _))
  (Variables|Default|SetStrafeRight _isa)
  (Utilities|Time|SetTimerbyEvent (delegate Custom|Strafe) 2.0 true))

(event Custom|StartFiring
  ;[1 1 1] Start Firing
  (if (Variables|Default|GetIsAttacking)
    (Utilities|FlowControl|DoOnce true :!label _label
      (:Completed
        (bind _returnvalue (Utilities|Time|SetTimerbyEvent (EventDispatchers|CreateEvent :!event FireWeapon) (Math|Random|RandomFloatinRange 0.2 1.0) true))
        (Variables|Default|SetShootTimer _returnvalue)))
    (else
      (Utilities|Time|ClearandInvalidateTimerbyHandle (Variables|Default|GetShootTimer))
      (goto _label Reset))))

(event EventBeginPlay
  (CallFunction|FetchClasses0))

(event EventTick
  (params (DeltaSeconds :type Float%20%28single-precision%29))
  (Utilities|FlowControl|Sequence
    (:then_1
      (CallFunction|StartFiring))))

(fn ConstructionScript
  (|CallParentFunction))

(fn FireWeapon
  (bind _shootpoint (Variables|Default|GetShootPoint))
  (bind _returnvalue (Transformation|GetWorldLocation _shootpoint))
  (bind _myplayer (CallFunction|GetPlayer))
  (Game|SpawnActorfromClass "/Game/MyBP/Actor/Projectile/BP_SkipShot.BP_SkipShot_C" (Math|Transform|MakeTransform _returnvalue (Math|Rotator|FindLookatRotation _returnvalue (Transformation|GetWorldLocation (Variables|/Game/FirstPerson/Blueprints/BP_FirstPersonCharacter.BP_FirstPersonCharacter_C|GetLookAT _myplayer))) "1.000000,1.000000,1.000000") "Undefined" "MultiplyWithRoot" 0 0 (Variables|Default|GetBaseDamage) self)
  (|CallParentFunction))

(fn FetchClasses0
  (bind _myplayer (CallFunction|GetPlayer))
  (Variables|Classes|SetMy%20Player_0 _myplayer))

(fn GetRandomLocationAroundPlayer
  (bind _direction (Utilities|GetDirection/Rotation))
  (AI|Navigation|MovetoLocation (AI|GetAIController (Pawn|GetController)) (Transformation|GetActorLocation (Variables|Classes|GetMy%20Player_0)) -1.0 true true true true 0)
  (if (> (Transformation|GetDistanceTo 0) (Variables|Default|GetAttackDistance))
    (Variables|Default|SetIsAttacking false)
    (Pawn|Input|AddMovementInput _direction 1.0 false)
    (else
      ;[0 0 0] Move back if near player
      (if (< (Transformation|GetDistanceTo (Variables|Classes|GetMy%20Player_0)) (- (Variables|Default|GetAttackDistance) 5e+02))
        (Pawn|Input|AddMovementInput _direction -1.0 false)
        (else
          ;[0 0 0] Strafe if near player
          (Pawn|Input|AddMovementInput (Math|Vector|GetRightVector (Math|Rotator|FindLookatRotation (Transformation|GetActorLocation) (Transformation|GetActorLocation (Variables|Classes|GetMy%20Player_0)))) (Math|Float|SelectFloat -0.5 0.5 (Variables|Default|GetStrafeRight)) false)
          (Variables|Default|SetIsAttacking true)))))
  (Transformation|SetActorRotation (.Rotation (Utilities|GetDirection/Rotation)))
  (return "0, 0, 0"))