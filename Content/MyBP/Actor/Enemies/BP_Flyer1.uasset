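; Flying enemy AI that chases the player, holds attack range and fires projectiles at them.
; Tick copies FlyerState to the blackboard and toggles a randomized-interval shoot timer from IsAttacking.
; ChasePlayer approaches, backs off or strafes by distance, with a looping timer flipping strafe direction.
; FireWeapon aims projectiles at the player's LookAT point, while a timed sphere overlap pushes it away from nearby Drone-tagged AI.
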(event Custom|Strafe
  ;[1 1 1] Strafe
  (bind _isa (Utilities|FlowControl|FlipFlop)
    (:A
      _)
    (:B
      _))
  (Variables|Default|SetStrafeRight _isa)
  (Utilities|Time|SetTimerbyEvent (delegate Custom|Strafe) 2.0 true))

(event Custom|StartFiring
  ;[1 1 1] Start Firing
  (if (Variables|Default|GetIsAttacking)
    (Utilities|FlowControl|DoOnce true :!label _label
      (:Completed
        (bind _returnvalue (Utilities|Time|SetTimerbyEvent (EventDispatchers|CreateEvent :!event FireWeapon) (Math|Random|RandomFloatinRange 0.2 1.0) true))
        (Variables|Default|SetShootTimer _returnvalue)))
    (else
      (Utilities|Time|ClearandInvalidateTimerbyHandle (Variables|Default|GetShootTimer))
      (goto _label Reset))))

(event EventBeginPlay
  (Utilities|FlowControl|Sequence
    (:then_0
      (Variables|Default|SetStartLocation (Transformation|GetActorLocation))
      (bind _myplayer (CallFunction|GetPlayer))
      (Variables|Default|SetMy%20Player_0 _myplayer))
    (:then_1
      (CallFunction|Strafe)
      (Utilities|Time|SetTimerbyFunctionName 0 "DetectOtherAI" 0.1 true))))

(event EventTick
  (params (DeltaSeconds :type Float%20%28single-precision%29))
  (bind _returnvalue (AI|GetBlackboard 0))
  (Utilities|FlowControl|Sequence
    (:then_0
      (Utilities|IsValid _returnvalue
        (:Is%20Valid
          (AI|Components|Blackboard|SetValueasEnum _returnvalue (Utilities|Name|MakeLiteralName "FlyerState") (Variables|Default|GetFlyerState)))))
    (:then_1
      (CallFunction|StartFiring))))

(fn ConstructionScript
  (|CallParentFunction))

(fn FireWeapon
  (bind _shootpoint (Variables|Default|GetShootPoint))
  (bind _returnvalue (Transformation|GetWorldLocation _shootpoint))
  (bind _asbp_first_person_character (Utilities|Casting|CastToBP_FirstPersonCharacter (Game|GetPlayerCharacter 0)))
  (Game|SpawnActorfromClass "/Game/MyBP/Actor/Projectile/Throwables/BP_Projectile.BP_Projectile_C" (Math|Transform|MakeTransform _returnvalue (Math|Rotator|FindLookatRotation _returnvalue (Transformation|GetWorldLocation (Variables|/Game/FirstPerson/Blueprints/BP_FirstPersonCharacter.BP_FirstPersonCharacter_C|GetLookAT _asbp_first_person_character))) "1.000000,1.000000,1.000000") "Undefined" "MultiplyWithRoot" 0 0 self)
  (|CallParentFunction))

(fn DetectOtherAI
  (bind _outactors (Collision|SphereOverlapActors (Transformation|GetActorLocation) 3e+02 (Utilities|Array|MakeArray "ObjectTypeQuery3") "/Game/MyBP/Actor/Enemies/BP_AIMaster.BP_AIMaster_C" (Utilities|Array|MakeArray self 0)))
  (for _array_element _outactors
    (if (Actor|ActorHasTag _array_element "Drone")
      (Pawn|Input|AddMovementInput (Math|Rotator|GetRotationXVector (Math|Rotator|MakeRotator (.roll (Math|Rotator|FindLookatRotation (Transformation|GetActorLocation) (Transformation|GetActorLocation _array_element))) (.pitch (Math|Rotator|FindLookatRotation (Transformation|GetActorLocation) (Transformation|GetActorLocation _array_element))) (.yaw (Math|Rotator|FindLookatRotation (Transformation|GetActorLocation) (Transformation|GetActorLocation _array_element))))) -1.0 false))))

(fn ChasePlayer
  (bind _direction (Utilities|ChaseLocationRotation))
  (switch Utilities|FlowControl|Switch|SwitchonE_FlyerChaseState (Variables|Default|GetChaseStates)
    (:NewEnumerator1
      (if (> (Transformation|GetDistanceTo (Variables|Default|GetMy%20Player_0)) (Variables|Default|GetAttackDistance))
        (Variables|Default|SetIsAttacking false)
        (Pawn|Input|AddMovementInput _direction 1.0 false)
        (else
          ;[0 0 0] Move back if near player
          (if (< (Transformation|GetDistanceTo (Variables|Default|GetMy%20Player_0)) (- (Variables|Default|GetAttackDistance) 5e+02))
            (Pawn|Input|AddMovementInput _direction -1.0 false)
            (else
              ;[0 0 0] Strafe if near player
              (Pawn|Input|AddMovementInput (Math|Vector|GetRightVector (Math|Rotator|FindLookatRotation (Transformation|GetActorLocation) (Transformation|GetActorLocation (Variables|Default|GetMy%20Player_0)))) (Math|Float|SelectFloat -0.5 0.5 (Variables|Default|GetStrafeRight)) false)
              (Variables|Default|SetIsAttacking true)))))
      (Transformation|SetActorRotation (.Rotation (Utilities|ChaseLocationRotation))))))