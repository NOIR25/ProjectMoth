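; Base enemy character that takes damage, reacts to player launches and pulls, and reports hits, deaths and combo tags to the game mode.
; AC_Damagable handles health, with incoming damage scaled by a debuff-driven multiplier.
; Elemental hits set bitflag debuffs: Heat stacks spawn DOT and spreading combust effect actors, Magic launches enemies weightless, while Goo and Lightning only draw debug spheres.
; Attack functions are empty hooks.
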(event OnDeath(AC_Damagable)
  (bind _mygamemode (CallFunction|GetGM))
  (Class|BPIGlobalEvents|EnemyFelled(Message) _mygamemode (Variables|Default|GetEnemyType) self)
  (Niagara|SpawnSystematLocation "/Game/MyBP/VFX/KillEffect.KillEffect" (Transformation|GetActorLocation) "0, 0, 0" "1.000000,1.000000,1.000000" true true "AutoRelease")
  (Default|CallOnDeath))

(event OnBlocked(AC_Damagable)
  (params (CanBeParried :type Boolean)))

(event OnDamageResponse(AC_Damagable)
  (params (DamageResponse :type E_DamageResponse%20Enum :default "NewEnumerator0"))
  (bind _my_gamemode (Variables|Default|GetMy%20Gamemode)
    (:then
      (Default|CallOnEnemyHit _my_gamemode)
      (switch Utilities|FlowControl|Switch|SwitchonE_DamageResponse DamageResponse
        (:NewEnumerator0
          (Development|PrintString "None"))
        (:NewEnumerator1
          (Development|PrintString "Hit Reaction")
          (Components|Activation|Activate (Variables|Default|GetNiagara) false)
          (Rendering|Material|SetOverlayMaterial (Variables|Character|GetMesh) "/Game/MyBP/VFX/M_PainOverlay.M_PainOverlay" :!class /Script/Engine.MeshComponent)
          (Utilities|FlowControl|Delay 0.2)
          (Rendering|Material|SetOverlayMaterial (Variables|Character|GetMesh) 0 :!class /Script/Engine.MeshComponent))))
    (:else)))

(event Custom|PullToPlayer
  (params (Location :type Vector))
  (bind _alpha (Timeline|PullTo PlayFromStart)
    (:Update
      (Transformation|SetWorldLocation (Variables|Collision|GetCapsuleComponent) (Math|Vector|Lerp(Vector) (Transformation|GetWorldLocation (Variables|Collision|GetCapsuleComponent)) Location _alpha) false false))))

(event Custom|AllowDeath
  (for _array_element (Actor|GetAttachedActors true true)
    (Actor|DestroyActor _array_element))
  (Actor|DestroyActor))

(event Custom|ClearHeatDebuff
  ;[0 0 0] Clear Heat Debuffs
  (Variables|Default|SetDamageRecievedMultiplier 1.0)
  (bind _newflags (CallFunction|RemoveDebuffFlag (Variables|DebuffSystem|GetActiveDebuffFlags) 1))
  (Variables|DebuffSystem|SetActiveDebuffFlags _newflags)
  (Development|PrintString "Default Heat Damaged Removed")
  (Utilities|Time|ClearandInvalidateTimerbyHandle (Variables|Element-Heat|GetHeatDOTTimer)))

(event EventBeginPlay
  (CallFunction|FetchClasses))

(event EventDefaultAttack
  (Development|PrintString "ATTACK!" true true "(R=1.000000,G=0.029149,B=0.000000,A=1.000000)")
  (CallFunction|CallDefaultAttack))

(event EventLaunchSlam
  (params (LaunchForce :type Vector :default "0, 0, 0"))
  (Character|LaunchCharacter LaunchForce true true)
  (GameplayTags|AddGameplayTag (Variables|Default|GetGameplayTags) "(TagName=\"ComboBuffs.Movement.EnemyLifted\")" :!class /Script/GameplayTags.BlueprintGameplayTagLibrary)
  (bind _my_gamemode (Variables|Default|GetMy%20Gamemode)
    (:then
      (Default|CheckEnemyComboTags _my_gamemode self))
    (:else)))

(event EventProcElementalDamage
  (params (Success :type Boolean) (ElementFlag :type Integer))
  (Debuffs-Default|SetDebuffDefaults ElementFlag)
  (if Success
    (bind _newflags (CallFunction|AddDebuffFlag (Variables|DebuffSystem|GetActiveDebuffFlags) ElementFlag))
    (bind _output_get (Variables|DebuffSystem|SetActiveDebuffFlags _newflags))
    (CallFunction|CallDebuffs _output_get)))

(event EventOnLanded
  (params (Hit :type Hit%20Result%20Structure%20%28by%20ref%29))
  (GameplayTags|RemoveGameplayTag (Variables|Default|GetGameplayTags) "(TagName=\"ComboBuffs.Movement.EnemyLifted\")" :!class /Script/GameplayTags.BlueprintGameplayTagLibrary)
  (bind _mygamemode (CallFunction|GetGM))
  (Default|CheckEnemyComboTags _mygamemode self))

(event EventTick
  (params (DeltaSeconds :type Float%20%28single-precision%29)))

(fn ConstructionScript)

(fn FireWeapon)

(fn CallDebuffs
  (params (DebuffFlags :type Integer))
  (bind _returnvalue (Transformation|GetActorLocation))
  (Utilities|FlowControl|Sequence
    (:then_0
      (bind _isset (CallFunction|HasDebuffFlag DebuffFlags 1))
      (if _isset
        (Development|PrintString "Call Fire Debuff")
        (Debuffs-Heat|CallHeatDebuffs)))
    (:then_1
      (bind _isset_2 (CallFunction|HasDebuffFlag DebuffFlags 2))
      (if _isset_2
        (Development|PrintString "Call Goo Debuff")
        (Rendering|Debug|DrawDebugSphere _returnvalue 5e+01 12 "(R=0.014731,G=1.000000,B=0.000000,A=1.000000)" 3.0 2.0)
        (return)))
    (:then_2
      (bind _isset_3 (CallFunction|HasDebuffFlag DebuffFlags 4))
      (if _isset_3
        (Development|PrintString "Call Lightning Debuff")
        (Rendering|Debug|DrawDebugSphere _returnvalue 5e+01 12 "(R=0.981443,G=1.000000,B=0.000000,A=1.000000)" 3.0 2.0)
        (return)))
    (:then_3
      (bind _isset_4 (CallFunction|HasDebuffFlag DebuffFlags 8))
      (if _isset_4
        (Development|PrintString "Call Magic Debuff")
        (Rendering|Debug|DrawDebugSphere _returnvalue 5e+01 12 "(R=1.000000,G=0.011788,B=0.922670,A=1.000000)" 3.0 2.0)
        (Debuffs-Magic|CallMagicDebuffs)
        (return)))))

(fn RemoveAllAffixes
  (params (DebuffFlags :type Integer))
  (Utilities|FlowControl|Sequence
    (:then_0
      (CallFunction|RemoveDebuffFlag DebuffFlags 1))
    (:then_1
      (CallFunction|RemoveDebuffFlag DebuffFlags 2))
    (:then_2
      (CallFunction|RemoveDebuffFlag DebuffFlags 4))
    (:then_3
      (CallFunction|RemoveDebuffFlag DebuffFlags 8))))

(fn HeatDebuffCombust
  (bind _returnvalue (Math|Random|RandomFloatinRange -5e+02 5e+02))
  (bind _myplayer (CallFunction|GetPlayer))
  (bind _outactors (Collision|SphereOverlapActors (Transformation|GetActorLocation) (Variables|DebuffSystem|GetAOE%20Radius) (Utilities|Array|MakeArray "ObjectTypeQuery3") 0 (Utilities|Array|MakeArray self _myplayer)))
  (Rendering|Debug|DrawDebugSphere (Transformation|GetActorLocation) (Variables|DebuffSystem|GetAOE%20Radius) 12 "(R=1.000000,G=0.123857,B=0.000000,A=1.000000)" 5.0 2.0)
  (for _array_element _outactors
    (Class|BPIEnemy|LaunchSlam(Message) _array_element (Math|Vector|MakeVector _returnvalue _returnvalue (Math|Random|RandomFloatinRange 2.5e+02 7.5e+02)))
    (Class|BPIEnemy|ProcElementalDamage(Message) _array_element (Math|Random|RandomBoolwithWeight (Variables|DebuffSystem|GetChanceToSpread)) 1)
    (Class|BPIDamagable|TakeDamage(Message) _array_element (Utilities|Struct|MakeS_DamageInfo (Variables|DebuffSystem|GetSpreadDamage) "NewEnumerator3" "NewEnumerator4")))
  (CallFunction|TakeDamage (Utilities|Struct|MakeS_DamageInfo (Variables|DebuffSystem|GetAOEDamage) "NewEnumerator3" "NewEnumerator4"))
  (return))

(fn CallHeatDebuffs
  (bind _output_get (Variables|Element-Heat|SetHeatStack (Math|Integer|Clamp(Integer) (+ (Variables|Element-Heat|GetHeatStack) 1) 0 (LocalVariables|GetMaxHeatStacks))))
  (Math|Integer|CompareInt _output_get
    (:>
      (bind _returnvalue (Game|SpawnActorfromClass "/Game/MyBP/Actor/Elemental/BP_Effects_HeatDOT.BP_Effects_HeatDOT_C" (Transformation|GetActorTransform) "AlwaysSpawn" "MultiplyWithRoot" 0 (Variables|Element-Heat|GetHeatDOT) 0.0 0))
      (Transformation|AttachActorToActor _returnvalue self "None" "SnapToTarget" "SnapToTarget" "SnapToTarget" true)
      (Math|Integer|CompareInt (Variables|Element-Heat|GetHeatStack) (LocalVariables|GetMaxHeatStacks)
        (:>
          (bind _returnvalue_2 (Game|SpawnActorfromClass "/Game/MyBP/Actor/Elemental/BP_Effects_HeatCombust.BP_Effects_HeatCombust_C" (Transformation|GetActorTransform) "AlwaysSpawn" "MultiplyWithRoot" 0 (Variables|DebuffSystem|GetAOE%20Radius) (Variables|DebuffSystem|GetAOEDamage) (Variables|DebuffSystem|GetChanceToSpread) (Variables|DebuffSystem|GetSpreadDamage) 0.0 1.0 0 :!label _label))
          (Transformation|AttachActorToActor _returnvalue_2 self "None" "SnapToTarget" "SnapToTarget" "SnapToTarget" true)
          (Variables|Element-Heat|SetHeatStack 0))
        (:==
          (goto _label))
        (:<
          (Development|PrintString "No enough stacks"))))
    (:==
      (Variables|Element-Heat|SetHeatStack 0 :!label _label_2))
    (:<
      (goto _label_2))))

(fn HeatDebuffSlowBurn
  (CallFunction|TakeDamage (Utilities|Struct|MakeS_DamageInfo (Variables|Element-Heat|GetHeatDOT) "NewEnumerator4" "NewEnumerator3"))
  (Utilities|FlowControl|DoOnce false
    (:Completed
      (Niagara|SpawnSystemAttached 0 (Variables|Character|GetMesh) "" (Transformation|GetActorLocation) "0, 0, 0" "KeepRelativeOffset" false false))))

(fn MagicDebuffFloater
  (bind _returnvalue (Math|Random|RandomFloatinRange -5e+02 5e+02))
  (CallFunction|LaunchSlam (Math|Vector|MakeVector _returnvalue _returnvalue 2e+02))
  (Variables|/Script/Engine.CharacterMovementComponent|SetGravityScale (Variables|Character|GetCharacterMovement) 0.0)
  (GameplayTags|AddGameplayTag (Variables|Default|GetGameplayTags) "(TagName=\"ComboBuffs.Movement.EnemyLifted\")" :!class /Script/GameplayTags.BlueprintGameplayTagLibrary)
  (Utilities|Time|SetTimerbyEvent (EventDispatchers|CreateEvent :!event MagicDebuffClearFloater) (Variables|Element-Magic|GetMagicFloaterTime)))

(fn CallMagicDebuffs
  (bind _output_get (Variables|Element-Magic|SetMagicStack (Math|Integer|Clamp(Integer) (+ (Variables|Element-Magic|GetMagicStack) 1) 0 (LocalVariables|GetMaxMagicStacks))))
  (Math|Integer|CompareInt _output_get
    (:>
      (Debuffs-Magic|MagicDebuffFloater))))

(fn MagicDebuffClearFloater
  (Variables|/Script/Engine.CharacterMovementComponent|SetGravityScale (Variables|Character|GetCharacterMovement) 1.0))

(fn DefaultHeatDamage
  (Variables|Default|SetDamageRecievedMultiplier 1.1)
  (Development|PrintString "Default Heat Damaged Added"))

(fn SetDebuffDefaults
  (params (DebuffFlag :type Integer))
  (Utilities|FlowControl|Sequence
    (:then_0
      (bind _isset (CallFunction|HasDebuffFlag DebuffFlag 1))
      (if _isset
        (Debuffs-Heat|DefaultHeatDamage)
        (Utilities|Time|SetTimerbyEvent (EventDispatchers|CreateEvent :!event Custom|ClearHeatDebuff) (Variables|Default|GetHeatDebuffDuration)))
      (return))
    (:then_1
      (bind _isset_2 (CallFunction|HasDebuffFlag DebuffFlag 2))
      (if _isset_2
        _
        (else
          _)))
    (:then_2
      (bind _isset_3 (CallFunction|HasDebuffFlag DebuffFlag 4))
      (if _isset_3
        _
        (else
          _)))
    (:then_3
      (bind _isset_4 (CallFunction|HasDebuffFlag DebuffFlag 8))
      (if _isset_4
        _
        (else
          _))))
  (return))

(fn LookatPlayer
  (params (TurnRate :type Float%20%28single-precision%29) (Target :type Actor%20Object%20Reference))
  (return (Math|Interpolation|RInterpTo (Transformation|GetActorRotation) (Math|Rotator|FindLookatRotation (Transformation|GetActorLocation) (Transformation|GetActorLocation Target)) (Utilities|Time|GetWorldDeltaSeconds) TurnRate)))

(fn FetchClasses
  (Utilities|FlowControl|Sequence
    (:then_0
      (bind _mygamemode (CallFunction|GetGM))
      (Variables|Default|SetMy%20Gamemode _mygamemode))))

(fn CallDefaultAttack)

(fn CheckNumpadEntry
  (return false 0))

(fn GetCurrentHealth
  (return (Variables|/Game/MyBP/DamageSystem/AC_Damagable.AC_Damagable_C|GetHealth (Variables|Default|GetAC_Damagable))))

(fn GetMaxhealth
  (return (Variables|/Game/MyBP/DamageSystem/AC_Damagable.AC_Damagable_C|GetCurrentMaxHealth (Variables|Default|GetAC_Damagable))))

(fn PullTowardsPlayer
  (params (PullToLocation :type Vector :default "0, 0, 0"))
  (CallFunction|PulltoPlayer PullToLocation)
  (return false))

(fn RestoreHealth
  (params (HealAmount :type Float%20%28double-precision%29))
  (bind _newhealth (Default|Heal (Variables|Default|GetAC_Damagable) HealAmount))
  (return _newhealth))

(fn RestoreSpite
  (params (Heal%20Amount :type Float%20%28double-precision%29))
  (return 0.0))

(fn TakeDamage
  (params (Damage%20Info :type S%20Damage%20Info%20Structure))
  (bind (_damageamount _damagetype _damageresponse _shoulddamageinvincible _canbeblocked _canbeparried _shouldforceinterrupt) (Utilities|Struct|BreakS_DamageInfo Damage%20Info))
  (bind _damagerecievedmultiplier (Variables|Default|GetDamageRecievedMultiplier))
  (bind _returnvalue (* _damageamount _damagerecievedmultiplier))
  (Development|PrintString (Utilities|String|ToString(Float) _returnvalue))
  (bind _wasdamaged (Default|TakeDamage (Variables|Default|GetAC_Damagable) (Utilities|Struct|MakeS_DamageInfo _returnvalue _damagetype _damageresponse _shoulddamageinvincible _canbeblocked _canbeparried _shouldforceinterrupt)))
  (return _wasdamaged))