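; Flying drone enemy that shoots projectiles at the player and can dive in as a suicide bomber.
; Tick mirrors FlyerState to the Blackboard and toggles randomly timed firing from IsAttacking, while timers flip strafe direction and push it away from nearby drones.
; ChasePlayer speeds up within attack range and freezes the tracked player location.
; Explode then polls until the drone reaches that point, damaging overlapping pawns and itself.
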(event Custom|Strafe
  ;[1 1 1] Strafe
  (bind _isa (Utilities|FlowControl|FlipFlop)
    (:A
      _)
    (:B
      _))
  (Variables|Default|SetStrafeRight _isa)
  (Utilities|Time|SetTimerbyEvent (delegate Custom|Strafe) 2.0 true))

(event Custom|StartFiring
  ;[1 1 1] Start Firing
  (if (Variables|Default|GetIsAttacking)
    (Utilities|FlowControl|DoOnce true :!label _label
      (:Completed
        (bind _returnvalue (Utilities|Time|SetTimerbyEvent (EventDispatchers|CreateEvent :!event FireWeapon) (Math|Random|RandomFloatinRange 0.2 1.0) true))
        (Variables|Default|SetShootTimer _returnvalue)))
    (else
      (Utilities|Time|ClearandInvalidateTimerbyHandle (Variables|Default|GetShootTimer))
      (goto _label Reset))))

(event Custom|Explode
  (bind _returnvalue (Transformation|GetActorLocation))
  (Utilities|FlowControl|Delay 0.0 :!label _label)
  (if (Utilities|Operators|EqualEqual (Transformation|GetActorLocation) (Variables|Default|GetPlayerLocation) 3e+01)
    (bind _outactors (Collision|SphereOverlapActors _returnvalue 5e+02 (Utilities|Array|MakeArray "ObjectTypeQuery3") 0 (Utilities|Array|MakeArray self)))
    (Rendering|Debug|DrawDebugSphere _returnvalue 5e+02 12 "(R=1.000000,G=0.032086,B=0.000000,A=1.000000)" 3.0 2.0)
    (for _array_element _outactors
      (Class|BPIDamagable|TakeDamage(Message) _array_element (Utilities|Struct|MakeS_DamageInfo (Variables|Default|GetBaseDamage) "NewEnumerator3" "NewEnumerator4" true)))
    ;[0 0 0] Damage Self
    (Default|TakeDamage (Variables|Default|GetAC_Damagable) (Utilities|Struct|MakeS_DamageInfo 99999.0 "NewEnumerator3" "NewEnumerator4"))
    (else
      (goto _label))))

(event EventBeginPlay
  (Utilities|FlowControl|Sequence
    (:then_0
      (Variables|Default|SetStartLocation (Transformation|GetActorLocation))
      (bind _myplayer (CallFunction|GetPlayer))
      (Variables|Default|SetMy%20Player_0 _myplayer))
    (:then_1
      (CallFunction|Strafe)
      (Utilities|Time|SetTimerbyFunctionName 0 "DetectOtherAI" 0.1 true)
      (bind _returnvalue (Utilities|Time|SetTimerbyEvent (EventDispatchers|CreateEvent :!event GetPlayerLocation) (Variables|Default|GetLocationUpdateSpeed) true))
      (Variables|Default|SetPlayerLocationTimer _returnvalue))))

(event EventTick
  (params (DeltaSeconds :type Float%20%28single-precision%29))
  (bind _returnvalue (AI|GetBlackboard 0))
  (Utilities|FlowControl|Sequence
    (:then_0
      (Utilities|IsValid _returnvalue
        (:Is%20Valid
          (AI|Components|Blackboard|SetValueasEnum _returnvalue (Utilities|Name|MakeLiteralName "FlyerState") (Variables|Default|GetFlyerState)))))
    (:then_1
      (CallFunction|StartFiring))))

(fn ConstructionScript
  (|CallParentFunction))

(fn FireWeapon
  (bind _shootpoint (Variables|Default|GetShootPoint))
  (bind _returnvalue (Transformation|GetWorldLocation _shootpoint))
  (bind _asbp_first_person_character (Utilities|Casting|CastToBP_FirstPersonCharacter (Game|GetPlayerCharacter 0)))
  (Game|SpawnActorfromClass "/Game/MyBP/Actor/Projectile/BP_Projectile.BP_Projectile_C" (Math|Transform|MakeTransform _returnvalue (Math|Rotator|FindLookatRotation _returnvalue (Transformation|GetWorldLocation (Variables|/Game/FirstPerson/Blueprints/BP_FirstPersonCharacter.BP_FirstPersonCharacter_C|GetLookAT _asbp_first_person_character))) "1.000000,1.000000,1.000000") "Undefined" "MultiplyWithRoot" 0 0 self)
  (|CallParentFunction))

(fn DetectOtherAI
  (bind _outactors (Collision|SphereOverlapActors (Transformation|GetActorLocation) 3e+02 (Utilities|Array|MakeArray "ObjectTypeQuery3") "/Game/MyBP/Actor/Enemies/BP_AIMaster.BP_AIMaster_C" (Utilities|Array|MakeArray self 0)))
  (for _array_element _outactors
    (if (Actor|ActorHasTag _array_element "Drone")
      (Pawn|Input|AddMovementInput (Math|Rotator|GetRotationXVector (Math|Rotator|MakeRotator (.roll (Math|Rotator|FindLookatRotation (Transformation|GetActorLocation) (Transformation|GetActorLocation _array_element))) (.pitch (Math|Rotator|FindLookatRotation (Transformation|GetActorLocation) (Transformation|GetActorLocation _array_element))) (.yaw (Math|Rotator|FindLookatRotation (Transformation|GetActorLocation) (Transformation|GetActorLocation _array_element))))) -1.0 false))))

(fn GetPlayerLocation
  (Variables|Default|SetPlayerLocation (Transformation|GetActorLocation (Variables|Default|GetMy%20Player_0)))
  (return))

(fn ChasePlayer
  (switch Utilities|FlowControl|Switch|SwitchonE_FlyerChaseState (Variables|Default|GetChaseStates)
    (:NewEnumerator1
      (if (> (Transformation|GetDistanceTo (Variables|Default|GetMy%20Player_0)) (Variables|Default|GetAttackDistance))
        (Variables|/Script/Engine.CharacterMovementComponent|SetMaxFlySpeed (Variables|Character|GetCharacterMovement) 6e+02)
        (else
          (Variables|/Script/Engine.CharacterMovementComponent|SetMaxFlySpeed (Variables|Character|GetCharacterMovement) 1.5e+03)
          (Utilities|Time|ClearandInvalidateTimerbyHandle (Variables|Default|GetPlayerLocationTimer))
          (CallFunction|Explode)))
      (Pawn|Input|AddMovementInput (.Direction (Utilities|ChaseLocationRotation)) 1.0 false)
      (Transformation|SetActorRotation (.Rotation (Utilities|ChaseLocationRotation))))))