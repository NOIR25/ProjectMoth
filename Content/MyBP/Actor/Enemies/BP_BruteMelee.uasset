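; Brute melee enemy Blueprint that caches the player on BeginPlay and chases them by issuing AI MoveTo every Tick.
; Its default attack runs a small debug-drawn sphere overlap at MeleePoint, damages Player-tagged pawns and then calls the parent attack.
; A FireWeapon override spawns BP_SkipShot aimed at the player.
; Strafe, retreat and timed-shooting logic remains, but its event-graph wiring is disconnected or empty.
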(event Custom|Strafe
  ;[1 1 1] Strafe
)

(event Custom|StartFiring
  ;[1 1 1] Start Firing
)

(event EventBeginPlay
  (CallFunction|FetchClasses0))

(event EventTick
  (params (DeltaSeconds :type Float%20%28single-precision%29))
  (AI|AIMoveTo self "0, 0, 0" (Variables|Classes|GetMy%20Player) 1.5e+02 false))

(fn ConstructionScript
  (|CallParentFunction))

(fn FireWeapon
  (bind _shootpoint (Variables|Default|GetShootPoint))
  (bind _returnvalue (Transformation|GetWorldLocation _shootpoint))
  (bind _myplayer (CallFunction|GetPlayer))
  (Game|SpawnActorfromClass "/Game/MyBP/Actor/Projectile/BP_SkipShot.BP_SkipShot_C" (Math|Transform|MakeTransform _returnvalue (Math|Rotator|FindLookatRotation _returnvalue (Transformation|GetWorldLocation (Variables|/Game/FirstPerson/Blueprints/BP_FirstPersonCharacter.BP_FirstPersonCharacter_C|GetLookAT _myplayer))) "1.000000,1.000000,1.000000") "Undefined" "MultiplyWithRoot" 0 0 (Variables|Default|GetBaseDamage) self)
  (|CallParentFunction))

(fn FetchClasses0
  (bind _myplayer (CallFunction|GetPlayer))
  (Variables|Classes|SetMy%20Player _myplayer))

(fn CallDefaultAttack
  (bind _meleepoint (Variables|Default|GetMeleePoint))
  (bind _returnvalue (Transformation|GetWorldLocation _meleepoint))
  (bind _outactors (Collision|SphereOverlapActors _returnvalue 3e+01 (Utilities|Array|MakeArray "ObjectTypeQuery3") 0 (Utilities|Array|MakeArray self)))
  (Rendering|Debug|DrawDebugSphere _returnvalue 3e+01 12 "(R=1.000000,G=1.000000,B=1.000000,A=1.000000)" 2.0 1.0)
  (for _array_element _outactors
    (if (Actor|ActorHasTag _array_element "Player")
      (Class|BPIDamagable|TakeDamage(Message) _array_element (Utilities|Struct|MakeS_DamageInfo 0.2 "NewEnumerator1" "NewEnumerator1"))
      (|CallParentFunction))))

(fn GetRandomLocationAroundPlayer
  (bind _direction (Utilities|GetDirection/Rotation))
  (bind _my_player (Variables|Classes|GetMy%20Player)
    (:then
      (if (> (Transformation|GetDistanceTo _my_player) (Variables|Default|GetRetreatDistance))
        (Variables|Default|SetIsRetreating false)
        (Pawn|Input|AddMovementInput _direction 1.0 false)
        (else
          ;[0 0 0] Move back if near player
          (if (< (Transformation|GetDistanceTo (Variables|Classes|GetMy%20Player)) (- (Variables|Default|GetRetreatDistance) 5e+02))
            (Pawn|Input|AddMovementInput _direction -1.0 false)
            (else
              ;[0 0 0] Strafe if near player
              (Pawn|Input|AddMovementInput (Math|Vector|GetRightVector (Math|Rotator|FindLookatRotation (Transformation|GetActorLocation) (Transformation|GetActorLocation (Variables|Classes|GetMy%20Player)))) (Math|Float|SelectFloat -0.5 0.5 (Variables|Default|GetStrafeRight)) false)
              (Variables|Default|SetIsRetreating true)))))
      (Transformation|SetActorRotation (.Rotation (Utilities|GetDirection/Rotation)))
      (return "0, 0, 0"))
    (:else)))