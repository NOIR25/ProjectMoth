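; BP_Hider is an enemy actor that restores health to the player when it dies.
; It caches player 0 at BeginPlay and, on the AC_Damagable death event, sends that player a restore-health message with HealAmount.
; Its mesh starts with custom depth rendering on, and the Lookat and StopLookingat events switch it on and off.
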(event OnDeath(AC_Damagable)
  (Class|BPIDamagable|RestoreHealth(Message) (Variables|Default|GetMy%20Player_0) (Variables|Default|GetHeal%20Amount)))

(event EventBeginPlay
  (|CallParentFunction)
  (bind _myplayer (CallFunction|GetPlayer))
  (Variables|Default|SetMy%20Player_0 _myplayer)
  (Rendering|SetRenderCustomDepth (Variables|Character|GetMesh) true))

(event Collision|EventActorBeginOverlap
  (params (OtherActor :type Actor%20Object%20Reference))
  (|CallParentFunction OtherActor) ; This node is disabled and will not be called.\nDrag off pins to build functionality.
)

(event EventTick
  (params (DeltaSeconds :type Float%20%28single-precision%29))
  (|CallParentFunction DeltaSeconds) ; This node is disabled and will not be called.\nDrag off pins to build functionality.
)

(event EventStopLookingat
  (Rendering|SetRenderCustomDepth (Variables|Character|GetMesh) false))

(event EventLookat
  (params (interactor :type BP%20First%20Person%20Character%20Object%20Reference))
  (Rendering|SetRenderCustomDepth (Variables|Character|GetMesh) true))

(fn ConstructionScript
  (|CallParentFunction))