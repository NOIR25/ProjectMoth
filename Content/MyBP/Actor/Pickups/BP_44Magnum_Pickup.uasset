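; Pickup actor for the .44 Magnum that gives the player a weapon in slot 1.
; The construction script sets the skeletal mesh from GunData, and BeginPlay caches player 0.
; Pickup checks the Weapon.Slot1 gameplay tag, spawns the gun from GunData on the player, switches to primary, marks it equipped and destroys the actor.
; The parent Pickup logic is left unconnected, so this override replaces it.
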(event EventBeginPlay
  (bind _myplayer (CallFunction|GetPlayer))
  (Variables|Default|SetMy%20Player_0 _myplayer))

(fn ConstructionScript
  (Components|SkeletalMesh|SetSkeletalMeshAsset (Variables|Default|GetSkeletalMesh) (Variables|/Game/MyBP/Weapons/Data/ProceduralWeaponSystem/PDA_WeaponBase.PDA_WeaponBase_C|GetWeaponSkeletalMesh (Variables|Default|GetGunData)))
  (|CallParentFunction))

(fn Pickup
  (bind _my_player_0 (Variables|Default|GetMy%20Player_0))
  (if (GameplayTags|HasTag (Variables|Default|GetGameplayTags) "(TagName=\"Weapon.Slot1\")")
    (bind _spawnedweapon (Default|SpawnWeaponSlot1 _my_player_0 (Variables|Default|GetGunData)))
    (Default|CESwitchtoPrimary _my_player_0)
    (Variables|/Game/FirstPerson/Blueprints/BP_FirstPersonCharacter.BP_FirstPersonCharacter_C|SetEquippedWeapon (Variables|Default|GetMy%20Player_0) _spawnedweapon)
    (Actor|DestroyActor)))