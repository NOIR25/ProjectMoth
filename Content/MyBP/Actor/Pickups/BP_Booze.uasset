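; BP_Booze is a booze pickup actor that goes into the player's LH inventory when collected.
; Its Pickup override disables collision on both meshes, then snaps the actor onto the player and hides it rather than destroying it.
; It registers itself and its InventoryStats quantity through AddToLHInventory on player 0, then runs the parent Pickup logic.
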(event EventBeginPlay
  (|CallParentFunction) ; This node is disabled and will not be called.\nDrag off pins to build functionality.
)

(event Collision|EventActorBeginOverlap
  (params (OtherActor :type Actor%20Object%20Reference)))

(event EventTick
  (params (DeltaSeconds :type Float%20%28single-precision%29)))

(fn ConstructionScript
  (|CallParentFunction))

(fn Pickup
  ;[0.15 0.15 0.15 0.5] Attach to player and disable
  (Collision|SetCollisionEnabled (Variables|Default|GetStaticMesh) "NoCollision")
  (Transformation|AttachActorToActor self (Variables|Default|GetMy%20Player) "None" "SnapToTarget" "SnapToTarget" "SnapToTarget" true)
  (Rendering|SetActorHiddenInGame true)
  (bind _myplayer (CallFunction|GetPlayer))
  (Default|AddtoLHInventory _myplayer self (Utilities|Struct|BreakS_InventoryStats (Variables|Default|GetInventoryStats)))
  (|CallParentFunction))