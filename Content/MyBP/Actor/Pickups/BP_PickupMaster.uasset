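; BP_PickupMaster is a pickup actor, apparently a base class, that reacts when the player overlaps its sphere.
; Overlap shows an inventory popup on the player HUD, calls an empty Pickup function, then passes StartingAmmo to the player's PickupNewAmmo.
; BeginPlay caches player and HUD references after a short delay.
; It also exposes its inventory item, reports player input as disabled, and triggers the player's SmokeQuery on inventory use.
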(event OnComponentBeginOverlap(Sphere)
  (params (OverlappedComponent :type Primitive%20Component%20Object%20Reference) (OtherActor :type Actor%20Object%20Reference) (OtherComp :type Primitive%20Component%20Object%20Reference) (OtherBodyIndex :type Integer) (bFromSweep :type Boolean) (SweepResult :type Hit%20Result%20Structure%20%28by%20ref%29))
  (if (Actor|ActorHasTag OtherActor "Player")
    (bind _wbp_playerhud (Variables|/Game/MyBP/UI/BP_HUD.BP_HUD_C|GetWBP_PlayerHUD (Variables|Default|GetHUD))
      (:then
        (Class|BPIUI|InventoryPopups(Message) _wbp_playerhud (Variables|Default|GetInventoryItem) (Variables|Default|GetInventoryStats)))
      (:else
        _))
    (CallFunction|Pickup)
    (bind _myplayer (CallFunction|GetPlayer))
    (Default|PickupNewAmmo _myplayer (Variables|Default|GetStartingAmmo))))

(event EventBeginPlay
  (Utilities|FlowControl|Delay 0.1)
  (bind _myplayer (CallFunction|GetPlayer))
  (Variables|Default|SetMy%20Player _myplayer)
  (bind _hud (CallFunction|GetHUD))
  (Variables|Default|SetHUD _hud))

(event EventInventoryUseEvent
  (bind _myplayer (CallFunction|GetPlayer))
  (Default|SmokeQuery _myplayer))

(fn ConstructionScript)

(fn Pickup)

(fn GetInventoryItems
  (return (Variables|Default|GetInventoryItem)))

(fn IsPlayerInputEnabled?
  (return false))