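; BP_DoubleBarrel_Pickup is a weapon pickup that gives the player a gun in the secondary slot.
; Construction sets the skeletal mesh from its GunData, and BeginPlay caches player 0.
; Pickup checks the gameplay tags for Weapon.Slot2, then has the player spawn the gun in slot 2, switch to it, and destroys the pickup.
; The parent Pickup logic is left unconnected and never runs.
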(event EventBeginPlay
  (bind _myplayer (CallFunction|GetPlayer))
  (Variables|Default|SetMy%20Player_0 _myplayer))

(fn ConstructionScript
  (Components|SkeletalMesh|SetSkeletalMeshAsset (Variables|Default|GetSkeletalMesh) (Variables|/Game/MyBP/Weapons/Data/ProceduralWeaponSystem/PDA_WeaponBase.PDA_WeaponBase_C|GetWeaponSkeletalMesh (Variables|Default|GetGunData)))
  (|CallParentFunction))

(fn Pickup
  (bind _my_player_0 (Variables|Default|GetMy%20Player_0))
  (if (GameplayTags|HasTag (Variables|Default|GetGameplayTags) "(TagName=\"Weapon.Slot2\")")
    (Default|SpawnWeaponSlot2 _my_player_0 (Variables|Default|GetGunData))
    (Default|CESwitchtoSecondary _my_player_0)
    (Actor|DestroyActor)))