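; BP_SkipShot is a projectile that tolerates one impact, then deals area damage on the second and destroys itself.
; Sphere hit events increment a bounce counter; the second triggers a pawn overlap query within AoERadius that sends each result a TakeDamage message carrying a damage info struct.
; A debug sphere with a hard-coded radius, independent of AoERadius, marks the blast.
; The projectile also self-destructs after a fixed lifetime.
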(event OnComponentHit(Sphere)
  (params (HitComponent :type Primitive%20Component%20Object%20Reference) (OtherActor :type Actor%20Object%20Reference) (OtherComp :type Primitive%20Component%20Object%20Reference) (NormalImpulse :type Vector :default "0, 0, 0") (Hit :type Hit%20Result%20Structure%20%28by%20ref%29))
  (bind _returnvalue (Transformation|GetActorLocation))
  (Math|Integer|IncrementInt (Variables|Default|GetBounceBuffer)
    (:%20%20
      (if (> (Variables|Default|GetBounceBuffer) 1)
        (bind _outactors (Collision|SphereOverlapActors _returnvalue (Variables|Default|GetAoE%20Radius) (Utilities|Array|MakeArray "ObjectTypeQuery3") 0 (Utilities|Array|MakeArray self)))
        (Rendering|Debug|DrawDebugSphere _returnvalue 2.5e+02 12 "(R=1.000000,G=0.043376,B=0.000000,A=1.000000)" 0.0 2.0)
        (for _array_element _outactors
          (Class|BPIDamagable|TakeDamage(Message) _array_element (Utilities|Struct|MakeS_DamageInfo (Variables|Default|GetDamage) "NewEnumerator2" "NewEnumerator4")))
        (Actor|DestroyActor)))))

(event EventBeginPlay
  (bind _myplayer (CallFunction|GetPlayer))
  (Variables|Default|SetMy%20Player _myplayer)
  (Utilities|FlowControl|Delay 5.0)
  (Actor|DestroyActor))

(fn ConstructionScript)