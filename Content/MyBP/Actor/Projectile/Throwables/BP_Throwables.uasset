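; BP_Throwables is a throwable projectile actor with area-of-effect impact logic.
; On BeginPlay it caches player 0 so that hits on that player are ignored.
; Any other sphere hit gathers pawns within AoERadius, excluding the player, and draws a debug sphere.
; It passes those pawns to CallGrenadeEffects, which is an empty hook here, and never destroys itself.
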(event OnComponentHit(Sphere)
  (params (HitComponent :type Primitive%20Component%20Object%20Reference) (OtherActor :type Actor%20Object%20Reference) (OtherComp :type Primitive%20Component%20Object%20Reference) (NormalImpulse :type Vector :default "0, 0, 0") (Hit :type Hit%20Result%20Structure%20%28by%20ref%29))
  (bind _returnvalue (Transformation|GetActorLocation))
  (bind _aoe_radius (Variables|Default|GetAoE%20Radius))
  (if (!= OtherActor (Variables|Default|GetMy%20Player))
    (bind _outactors (Collision|SphereOverlapActors _returnvalue _aoe_radius (Utilities|Array|MakeArray "ObjectTypeQuery3") 0 (Utilities|Array|MakeArray (Variables|Default|GetMy%20Player))))
    (Rendering|Debug|DrawDebugSphere _returnvalue _aoe_radius 12 "(R=1.000000,G=0.048397,B=0.000000,A=1.000000)" 3.0 2.0)
    (CallFunction|CallGrenadeEffects _outactors)))

(event EventBeginPlay
  (bind _myplayer (CallFunction|GetPlayer))
  (Variables|Default|SetMy%20Player _myplayer))

(fn ConstructionScript)

(fn CallGrenadeEffects
  (params (HitActors :type Array%20of%20Actor%20Object%20References)))