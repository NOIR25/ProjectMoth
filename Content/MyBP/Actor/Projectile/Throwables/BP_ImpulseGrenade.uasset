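; Impulse grenade throwable that knocks the actors it hits into the air and damages them.
; Its CallGrenadeEffects function takes a list of hit actors and sends each a launch message with random horizontal force and fixed upward force, then a base-damage message.
; The grenade destroys itself afterward, and its event graph and construction script add no logic of their own.
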(event EventBeginPlay
  (|CallParentFunction) ; This node is disabled and will not be called.\nDrag off pins to build functionality.
)

(event Collision|EventActorBeginOverlap
  (params (OtherActor :type Actor%20Object%20Reference)))

(event EventTick
  (params (DeltaSeconds :type Float%20%28single-precision%29)))

(fn ConstructionScript
  (|CallParentFunction))

(fn CallGrenadeEffects
  (params (HitActors :type Array%20of%20Actor%20Object%20References))
  (bind _returnvalue (Math|Random|RandomFloatinRange -1e+03 1e+03))
  (for _array_element HitActors
    (Class|BPIEnemy|LaunchSlam(Message) _array_element (Math|Vector|MakeVector _returnvalue _returnvalue 7.5e+02))
    (Class|BPIDamagable|TakeDamage(Message) _array_element (Utilities|Struct|MakeS_DamageInfo (Variables|Default|GetBaseDamage) "NewEnumerator2" "NewEnumerator1")))
  (Actor|DestroyActor))