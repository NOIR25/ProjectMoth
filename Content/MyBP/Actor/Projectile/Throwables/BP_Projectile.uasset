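; Projectile actor fired from a weapon that damages enemies when its sphere component hits them.
; It caches player 0 on BeginPlay to ignore as a hit target, then sends BPI_Enemy actors a damage message using the source weapon's FinalDamage.
; The hit-result, weapon juice and DestroyActor calls are disconnected, so this graph never destroys the projectile.
; ShotFromWeapon's validity is checked only after that damage read, and the check leads nowhere.
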(event OnComponentHit(Sphere)
  (params (HitComponent :type Primitive%20Component%20Object%20Reference) (OtherActor :type Actor%20Object%20Reference) (OtherComp :type Primitive%20Component%20Object%20Reference) (NormalImpulse :type Vector :default "0, 0, 0") (Hit :type Hit%20Result%20Structure%20%28by%20ref%29))
  (if (!= OtherActor (Variables|Default|GetMy%20Player))
    (if (Utilities|DoesObjectImplementInterface OtherActor "/Game/MyBP/Interfaces/BPI_Enemy.BPI_Enemy_C")
      (Class|BPIDamagable|TakeDamage(Message) OtherActor (Utilities|Struct|MakeS_DamageInfo (Variables|/Game/MyBP/Weapons/BP_WeaponClass.BP_WeaponClass_C|GetFinalDamage (Variables|Default|GetShotFromWeapon)) "NewEnumerator2" "NewEnumerator1"))))
  (bind _shotfromweapon (Variables|Default|GetShotFromWeapon)
    (:then)
    (:else)))

(event EventBeginPlay
  (bind _myplayer (CallFunction|GetPlayer))
  (Variables|Default|SetMy%20Player _myplayer))

(fn ConstructionScript)