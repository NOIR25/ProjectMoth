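; Damageable actor component that manages health, healing and incoming damage for its owner.
; TakeDamage uses the CanBeDamaged macro to route a DamageInfo to blocked, damaged or ignored, based on death, invincibility and blocking.
; Damage lowers clamped health, then signals death or, if interruptable or forced, a damage response; blocked hits signal whether they can be parried.
; Heal adds health up to the current maximum while alive.
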(fn Heal
  (params (Amount :type Float%20%28double-precision%29))
  (if (not (Variables|Default|GetIsDead))
    (bind _output_get (Variables|Default|SetHealth (Math|Float|Clamp(Float) (+ Amount (Variables|Default|GetHealth)) -1.0 (Variables|Default|GetCurrentMaxHealth))))
    (return _output_get)))

(fn TakeDamage
  (params (DamageInfo :type S%20Damage%20Info%20Structure))
  (bind (_damageamount _damagetype _damageresponse _shoulddamageinvincible _canbeblocked _canbeparried _shouldforceinterrupt) (Utilities|Struct|BreakS_DamageInfo DamageInfo))
  (Utilities|CanbeDamaged _shoulddamageinvincible _canbeblocked
    (:BlockedDamage
      (Default|CallOnBlocked _canbeparried)
      (return false))
    (:DoDamage
      (bind _output_get (Variables|Default|SetHealth (Math|Float|Clamp(Float) (- (Variables|Default|GetHealth) _damageamount) 0.0 (Variables|Default|GetCurrentMaxHealth))))
      (if (<= _output_get 0.0)
        (Default|CallOnDeath)
        (return true)
        (elif (or (Variables|Default|GetIsInterruptable) _shouldforceinterrupt)
          (Default|CallOnDamageResponse _damageresponse)
          (return true))))
    (:NoDamage
      (return false))))