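; Player interaction component that detects and triggers objects implementing BPI_Interactions through camera-forward Visibility line traces.
; On BeginPlay it caches player, camera, controller, HUD and game mode references.
; Tick runs a long trace to send look-at and stop-looking messages, while IA_Interact runs a shorter debug-drawn trace to send tap-interact.
; A separate helper nudges the mouse cursor by scaled joystick input, although the traces ignore cursor position.
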(event Input|EnhancedActionEvents|EnhancedInputActionIA_Interact
  (params (ActionValue :type Boolean) (ElapsedSeconds :type Float%20%28double-precision%29) (TriggeredSeconds :type Float%20%28double-precision%29) (InputAction :type Input%20Action%20Object%20Reference :default "/Game/FirstPerson/Input/Actions/IA_Interact.IA_Interact"))
  ;[0 0 0] Checks for interactable objects on trace hit
  ; Calls Tap interact function
  (:Started
    (bind _outhit (Utilities|LineTracefromMousePosition 2.5e+02 "ForDuration"))
    (if (Utilities|DoesObjectImplementInterface (.HitActor (Collision|BreakHitResult _outhit)) "/Game/MyBP/Interfaces/BPI_Interactions.BPI_Interactions_C")
      (Variables|Actors|SetInteractingActor (.HitActor (Collision|BreakHitResult _outhit)))
      (Utilities|IsValid (Variables|FetchedClasses|GetMy%20Player)
        (:Is%20Valid
          (Class|BPIInteractions|TapInteract(Message) (Variables|Actors|GetInteractingActor) (Variables|FetchedClasses|GetMy%20Player))
          (Default|CallOnTapInteract))))))

(event EventBeginPlay
  (CallFunction|FetchClasses))

(event EventTick
  (params (DeltaSeconds :type Float%20%28single-precision%29))
  (bind _outhit (Utilities|LineTracefromMousePosition 5e+03 "None"))
  (if (Utilities|DoesObjectImplementInterface (.HitActor (Collision|BreakHitResult _outhit)) "/Game/MyBP/Interfaces/BPI_Interactions.BPI_Interactions_C")
    (bind _output_get (Variables|Actors|SetHoveredActor (.HitActor (Collision|BreakHitResult _outhit))))
    (Class|BPIInteractions|Lookat(Message) _output_get (Variables|FetchedClasses|GetMy%20Player))
    (else
      (Utilities|IsValid (Variables|Actors|GetHoveredActor)
        (:Is%20Valid
          (Class|BPIInteractions|StopLookingat(Message) (Variables|Actors|GetHoveredActor))
          (Variables|Actors|SetHoveredActor 0))))))

(fn FetchClasses
  (bind _returnvalue (Components|GetOwner))
  (bind _myplayer (Class|BPIClassFetcher|GetMyPlayer(Message) _returnvalue))
  (Variables|FetchedClasses|SetMy%20Player _myplayer)
  (bind _camera (Class|BPIClassFetcher|GetPlayerComponents(Message) _returnvalue))
  (Variables|Default|SetCamera _camera)
  (bind _mycontroller (CallFunction|GetPC))
  (Variables|FetchedClasses|SetMy%20Controller _mycontroller)
  (bind _hud (CallFunction|GetHUD))
  (Variables|FetchedClasses|SetHUD _hud)
  (bind _mygamemode (CallFunction|GetGM))
  (Variables|FetchedClasses|SetMy%20Gamemode _mygamemode))